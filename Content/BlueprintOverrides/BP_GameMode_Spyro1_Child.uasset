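; Child override of the Spyro 1 game mode that adds on-screen debug logging to player start selection.
; ChoosePlayerStart and FindPlayerStart call the parent implementation, print a timed colored message with the player path plus either the chosen start or the incoming name, then return the parent's result unchanged.
; BeginPlay, Tick and the construction script only forward to the parent.
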(event `self.ReceiveBeginPlay`
  (`parent.ReceiveBeginPlay`))

(event `self.ReceiveTick`
  (params (DeltaSeconds :type "Float (single-precision)"))
  (`parent.ReceiveTick` DeltaSeconds))

(fn `ChoosePlayerStart`
  (params (Player :type "Controller Object Reference"))
  (returns (ReturnValue :type "Actor Object Reference"))
  (bind _returnvalue (`parent.ChoosePlayerStart` Player))
  (`/Game/ModLoader/Blueprints/Widgets/Utility/BF_PrintText.BF_PrintString` (`KismetTextLibrary.Conv_TextToString` (`|FormatText` "Choosse Player Start \n \nPlayer {player} \nReturn Value {value}" (`KismetTextLibrary.Conv_StringToText` (`KismetSystemLibrary.GetPathName` Player)) (`KismetTextLibrary.Conv_StringToText` (`KismetSystemLibrary.GetPathName` _returnvalue)))) (struct :`G` 1.0 :`B` 0.737911 :`A` 1.0) 10.0)
  (return _returnvalue))

(fn `FindPlayerStart`
  (params (Player :type "Controller Object Reference") (IncomingName :type String))
  (returns (ReturnValue :type "Actor Object Reference"))
  (bind _returnvalue (`parent.FindPlayerStart` Player IncomingName))
  (`/Game/ModLoader/Blueprints/Widgets/Utility/BF_PrintText.BF_PrintString` (`KismetTextLibrary.Conv_TextToString` (`|FormatText` "Find player start \n \nPlayer {player} \nIncoming Name {name}" (`KismetTextLibrary.Conv_StringToText` (`KismetSystemLibrary.GetPathName` Player)) (`KismetTextLibrary.Conv_StringToText` IncomingName))) (struct :`G` 1.0 :`B` 0.737921 :`A` 1.0) 10.0)
  (return _returnvalue))

(fn `UserConstructionScript`
  (`parent.UserConstructionScript`))