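; Sparx health mod Blueprint that recolors Spyro according to the color of his dragonfly companion Sparx.
; Each tick it gets the playable Spyro, updates both eye power-up states and flags an active power-up by comparing the body mesh's material against five candidates.
; Without a power-up, it reads the Diffuse Map texture from Sparx's dynamic material and calls ChangeSpyroColor for the matching color, with a fallback branch.
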(event `GetSpyroSparx`
  (cast `/CPS1999_Spyro/Blueprints/BP_CPS1999_Playable` (`GameplayStatics.GetPlayerCharacter` 0)))

(event `self.ReceiveTick`
  (params (DeltaSeconds :type "Float (single-precision)"))
  (`self.GetSpyroSparx`)
  (`self.SetLeftEyePowerUp`)
  (`self.SetRightEyePowerUp`)
  (`self.GetPowerUp`)
  (if (not (`self.Powerup?`))
    (bind _asmaterial_instance_dynamic (cast `MaterialInstanceDynamic` (`PrimitiveComponent.GetMaterial` (`self.GetComponentByClass` (`self.Sparx`) "/Script/Engine.SkeletalMeshComponent") 1)))
    (bind _returnvalue (`MaterialInstanceDynamic.K2_GetTextureParameterValue` _asmaterial_instance_dynamic "Diffuse Map"))
    (if (== _returnvalue "/CPS1194_SparxNew/Textures/T_CPS1194_SparxNew_C.T_CPS1194_SparxNew_C")
      (`self.ChangeSpyroColor` null)
      (elif (== _returnvalue "/CPS1194_SparxNew/Textures/T_CPS1194_SparxNew_C_Blue.T_CPS1194_SparxNew_C_Blue")
        (`self.ChangeSpyroColor` null)
        (else
          (`self.ChangeSpyroColor` null))))))

(event `GetPowerUp`
  (bind _returnvalue (`PrimitiveComponent.GetMaterial` (`Character.Mesh` (`GameplayStatics.GetPlayerCharacter` 0)) 0))
  (if (== _returnvalue null)
    (set `self.Powerup?` true :!label _label)
    (elif (== _returnvalue null)
      (goto _label)
      (elif (== _returnvalue null)
        (goto _label)
        (elif (== _returnvalue null)
          (goto _label)
          (elif (== _returnvalue null)
            (goto _label)
            (else
              (set `self.Powerup?` false))))))))

(fn `UserConstructionScript`)