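; Ragdoll corpse actor that stands in for a dead actor, taking over its materials and simulating physics.
; In packaged builds it poses from a supplied animation, appears after a delay, then ragdolls; otherwise it previews from an idle pose.
; Tick follows the source mesh while visible.
; It destroys itself with the source's owner or after player death, which also ragdolls the player; damage and kill hooks only print debug text.
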(event `SetupMaterials`
  (bind _meshcomp (`self.MeshComp`))
  ;[1 1 1] Keep original materials from dead actor. This fixes burn material
  (`/Engine/EditorBlueprintResources/StandardMacros.IsValid` _meshcomp
    (:`Is Valid`
      (for (_array_element _array_index) (`MeshComponent.GetMaterials` _meshcomp)
        (`/Engine/EditorBlueprintResources/StandardMacros.IsValid` _array_element
          (:`Is Valid`
            (`PrimitiveComponent.SetMaterial` (`self.Mesh`) _array_index _array_element)))))))

(event `self.ReceiveTick`
  (params (DeltaSeconds :type "Float (single-precision)"))
  (bind _meshcomp (`self.MeshComp`))
  (`/Engine/EditorBlueprintResources/StandardMacros.IsValid` _meshcomp
    (:`Is Valid`
      (if (`SceneComponent.IsVisible` _meshcomp)
        (`self.K2_SetActorTransform` (`SceneComponent.K2_GetComponentToWorld` (`self.MeshComp`)))
        (else
          (`/Engine/EditorBlueprintResources/StandardMacros.DoOnce` false
            (:`Completed`
              (`PrimitiveComponent.SetSimulatePhysics` (`self.Mesh`) true))))))))

(event `MakeVisible`
  (`SceneComponent.SetHiddenInGame` (`self.Mesh`) false true))

(event `self.ReceiveBeginPlay`
  (bind _mesh (`self.Mesh`))
  (bind _animtoplay (`self.AnimToPlay`))
  (bind _mesh_2 (`self.Mesh`))
  (bind _returnvalue (`ActorComponent.GetOwner` (`self.MeshComp`)))
  (bind _sequencelength (`AnimSequenceBase.SequenceLength` _animtoplay))
  (if (`KismetSystemLibrary.IsPackagedForDistribution`)
    (`SkinnedMeshComponent.SetSkinnedAssetAndUpdate` (`self.Mesh`) (`self.Mesh_0`) true)
    (set `self.Tags` (`|MakeArray` (`self.tag`)))
    (add `PhasmidCharacter.OnDealDamageDelegate` (cast `/CharacterCommon/BaseClasses/BP_Base_Playable` (`GameplayStatics.GetPlayerCharacter` 0) :!pure true) (delegate `OnDealDamageDelegate_Event_0`))
    (add `PhasmidCharacter.OnDeathDelegate` (cast `/CharacterCommon/BaseClasses/BP_Base_Playable` (`GameplayStatics.GetPlayerCharacter` 0) :!pure true) (delegate `OnDeathDelegate_Event_0`)) ; Remove Ragdolls when spyro dies
    (add `self.OnDestroyed` _returnvalue (delegate `DestroyActors`))
    (add `self.OnEndPlay` _returnvalue (delegate `DestroyActors2`))
    (`/Game/ModLoader/Blueprints/Widgets/Utility/BF_PrintText.BF_PrintString` (`KismetStringLibrary.Concat_StrStr` "Spawned Corse For: " (`KismetSystemLibrary.GetDisplayName` (`ActorComponent.GetOwner` (`self.MeshComp`))) " Actor Tag: " (`KismetStringLibrary.Conv_NameToString` (`|GetArrayItem` (`self.Tags`)))) (struct :`R` 0.846873 :`G` 0.366253 :`B` 1.0 :`A` 1.0))
    (`self.SetupMaterials`)
    (`SkeletalMeshComponent.PlayAnimation` _mesh_2 _animtoplay false)
    (`SkeletalMeshComponent.SetPosition` _mesh_2 (`KismetMathLibrary.NormalizeToRange` _sequencelength 0.0 _sequencelength) false)
    (`SkeletalMeshComponent.SetPlayRate` _mesh_2 0.0)
    (`TextRenderComponent.K2_SetText` (`self.TextRender`) (`KismetTextLibrary.Conv_StringToText` (`KismetSystemLibrary.GetDisplayName` (`SkeletalMesh.PhysicsAsset` (`SkinnedMeshComponent.SkeletalMesh` (`self.Mesh`))))))
    (`KismetSystemLibrary.Delay` 1.0)
    (`self.MakeVisible`)
    (`PrimitiveComponent.SetSimulatePhysics` (`self.Mesh`) true)
    (else
      (`self.MakeVisible`)
      (`SkeletalMeshComponent.PlayAnimation` _mesh "/Game/Resources_Tests/NavTest/ThirdPersonBP/Animations/ThirdPersonIdle.ThirdPersonIdle" false)
      (`SkeletalMeshComponent.SetPosition` _mesh 3.0 false)
      (`SkeletalMeshComponent.SetPlayRate` _mesh 0.0)
      (`KismetSystemLibrary.Delay` 1.0)
      (`SkinnedMeshComponent.SetSkinnedAssetAndUpdate` (`self.Mesh`) (`self.Mesh_0`) true)
      (`PrimitiveComponent.SetSimulatePhysics` (`self.Mesh`) true))))

(event `DestroyActors` :!signature `self.OnDestroyed`
  (params (DestroyedActor :type "Actor Object Reference"))
  (`self.K2_DestroyActor` :!label _label))

(event `DestroyActors2` :!signature `self.OnEndPlay`
  (params (Actor :type "Actor Object Reference") (EndPlayReason :type "EEndPlayReason Enum" :default "Destroyed"))
  (goto _label))

(event `OnDealDamageDelegate_Event_0`
  (params (Actor :type "Actor Object Reference") (Payload :type "GameplayEventData Structure"))
  (bind (_eventtag _instigator _target) (break `GameplayEventData` Payload))
  (`/Game/ModLoader/Blueprints/Widgets/Utility/BF_PrintText.BF_PrintString` (`KismetStringLibrary.BuildString_Object` "" "Spyro Dealt Damage To:" _target (`KismetStringLibrary.Concat_StrStr` " \n" "With Tags:" (`BlueprintGameplayTagLibrary.GetDebugStringFromGameplayTag` _eventtag))) (struct :`R` 0.846873 :`G` 0.366253 :`B` 1.0 :`A` 1.0))
  (add `PhasmidCharacter.OnDeathDelegate` (cast `/CharacterCommon/BaseClasses/BP_Base_NPC` _target :!pure true) (delegate `CustomEvent_0`)))

(event `OnDeathDelegate_Event_0`
  (params (Actor :type "Actor Object Reference") (Payload :type "GameplayEventData Structure"))
  (`PrimitiveComponent.SetSimulatePhysics` (`Character.Mesh` (cast `/CharacterCommon/BaseClasses/BP_Base_Playable` (`GameplayStatics.GetPlayerCharacter` 0) :!pure true)) true)
  (`KismetSystemLibrary.Delay` 4.0)
  (`self.K2_DestroyActor`))

(event `CustomEvent_0`
  (params (Actor :type "Actor Object Reference") (Payload :type "GameplayEventData Structure"))
  (`/Game/ModLoader/Blueprints/Widgets/Utility/BF_PrintText.BF_PrintString` (`KismetStringLibrary.BuildString_Object` "" "Spyro Killed:" Actor) (struct :`R` 0.846873 :`G` 0.366253 :`B` 1.0 :`A` 1.0)))

(fn `UserConstructionScript`
  (`SkinnedMeshComponent.SetSkinnedAssetAndUpdate` (`self.Mesh`) (`self.Mesh_0`) true)
  (set `self.Tags` (`|MakeArray` (`self.tag`))))