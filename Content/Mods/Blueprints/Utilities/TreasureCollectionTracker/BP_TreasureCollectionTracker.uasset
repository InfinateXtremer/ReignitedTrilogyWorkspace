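; Mod utility actor that shows the current level's treasure collection progress on the Spyro player character.
; Every tick it normalizes collected treasure against the level total, writing the result to a material parameter collection scalar and the player mesh's "TreasureCollection" morph target.
; It also rechecks the player mesh each tick, creating a dynamic instance of the fireball Spyro material when slot 0 lacks one.
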(event `self.ReceiveTick`
  (params (DeltaSeconds :type "Float (single-precision)"))
  (`self.Checkmaterial`)
  (bind _level_name (message `/GameplayCommon/GameModes/GameStateInterface.get current level name` (`GameplayStatics.GetGameState`)))
  (set `self.CurrentLevel` _level_name)
  (bind _returnvalue (`FalconGameplayStatics.GetLevelInventoryTotalForType` "EIT_Treasure" (`self.CurrentLevel`)))
  (bind _returnvalue_2 (`FalconGameplayStatics.GetInventoryCollectedCountForType` "EIT_Treasure" (`self.CurrentLevel`)))
  (bind _returnvalue_3 (`KismetMathLibrary.NormalizeToRange` (`KismetMathLibrary.Conv_IntToDouble` _returnvalue_2) 0.0 (`KismetMathLibrary.Conv_IntToDouble` _returnvalue)))
  (`KismetMaterialLibrary.SetScalarParameterValue` "/Game/Mods/Blueprints/Utilities/TreasureCollectionTracker/MPC_TreasureCollection.MPC_TreasureCollection" "CollectionPercentage" _returnvalue_3)
  (`SkeletalMeshComponent.SetMorphTarget` (`self.Mesh`) "TreasureCollection" _returnvalue_3 true))

(event `Checkmaterial`
  (bind _asbp_cps1999_playable (cast `/CPS1999_Spyro/Blueprints/BP_CPS1999_Playable` (`GameplayStatics.GetPlayerCharacter` 0)))
  (bind _mesh (`Character.Mesh` _asbp_cps1999_playable))
  (set `self.Mesh` _mesh)
  (bind _asmaterial_instance_dynamic (cast `MaterialInstanceDynamic` (`PrimitiveComponent.GetMaterial` _mesh 0))
    (:`then`
      (set `self.Material` _asmaterial_instance_dynamic))
    (:`CastFailed`
      (`PrimitiveComponent.CreateDynamicMaterialInstance` _mesh 0 "/CPS1999_Spyro/Materials/MI_CPS1999_Spyro_Fireball.MI_CPS1999_Spyro_Fireball"))))

(fn `UserConstructionScript`)