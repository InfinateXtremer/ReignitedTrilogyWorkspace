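; Random mod actor that ties the player's survival to charging, going by its name and countdown damage.
; Each tick it reads the player character's charging state, playing the CountDown timeline while charging and reversing it otherwise.
; Whenever a timeline update reads zero or below, ApplyDamage applies a fixed damage effect to the player with a randomly picked damage tag.
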(event `self.ReceiveTick`
  (params (DeltaSeconds :type "Float (single-precision)"))
  (bind _asbp_cps1999_playable (cast `/CPS1999_Spyro/Blueprints/BP_CPS1999_Playable` (`GameplayStatics.GetPlayerCharacter` 0)))
  (bind _ischarging (`/CharacterCommon/BaseClasses/BP_Base_Playable.IGetIsCharging` _asbp_cps1999_playable))
  (if _ischarging
    (bind (_direction _newtrack_0) (`Timeline|CountDown` :!label _label)
      (:`Update`
        (if (<= (* _newtrack_0 60.0) 0.0)
          (`self.ApplyDamage`))))
    (else
      (goto _label :!via `Reverse`))))

(fn `UserConstructionScript`)