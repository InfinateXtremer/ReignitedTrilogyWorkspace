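; Harder Spyro mod Blueprint that periodically rains timed bombs on the player, with the Multiply key triggering the same wave manually.
; A looping timer or key press prints a message and spawns a batch of BP_TimedBomb actors owned by the player.
; CastRay traces upward from the player, then picks random points in a box oriented to the hit normal, or facing down below the trace end.
; Debug drawing shows the trace, box and points.
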(event `self.ReceiveBeginPlay`
  (`KismetSystemLibrary.K2_SetTimer` null "RainBombs" 10.0 true))

(event `Key|Multiply` :consume false :overrideparent false
  (params (Key :type "Key Structure"))
  (:`Pressed`
    (`/Game/ModLoader/Blueprints/Widgets/Utility/BF_PrintText.BF_PrintString` "Raining bombs" :!label _label)
    (for _ (range 21)
      (bind _randomlocationaboveplayer (`self.CastRay` (`|MakeArray` (`GameplayStatics.GetPlayerCharacter` 0) :!type "Actor Object Reference")))
      (`|SpawnActorFromClass` "/Game/Mods/Blueprints/HarderSpyro/RainingBombs/BP_TimedBomb.BP_TimedBomb_C" (`KismetMathLibrary.MakeTransform` _randomlocationaboveplayer) "Undefined" "OverrideRootScale" (`GameplayStatics.GetPlayerCharacter` 0) null))))

(event `RainBombs`
  (goto _label))

(fn `CastRay`
  (params (ExtraActorsToIgnore :type "Array of Actor Object Reference"))
  (returns (RandomLocationAbovePlayer :type "Vector Structure"))
  (locals (ObjectTypes :type "Array of EObjectTypeQuery Enum") (ActorsToIgnore :type "Array of Actor Object Reference") (RayEnd :type "Vector Structure" :default (0.0 0.0 0.0)) (RayStart :type "Vector Structure" :default (0.0 0.0 0.0)) (BoxExtent :type "Vector Structure" :default (50.0 500.0 500.0)) (HitNormal :type "Vector Structure") (HitVector :type "Vector Structure"))
  (bind _rayend (`local.RayEnd`))
  (bind _hitnormal (`local.HitNormal`))
  (bind _boxextent_x (`KismetMathLibrary.BreakVector` (`local.BoxExtent`)))
  (bind _returnvalue (`self.K2_GetActorLocation` (`GameplayStatics.GetPlayerCharacter` 0)))
  (bind _returnvalue_2 (`KismetMathLibrary.Conv_VectorToRotator` _hitnormal))
  (bind _returnvalue_3 (`KismetMathLibrary.TransformLocation` (`KismetMathLibrary.MakeTransform` (`local.HitVector`) _returnvalue_2) (`KismetMathLibrary.RandomPointInBoundingBox` (`KismetMathLibrary.MakeVector` _boxextent_x) (`local.BoxExtent`))))
  (set `local.ActorsToIgnore` ExtraActorsToIgnore)
  (set `local.RayStart` _returnvalue)
  (set `local.RayEnd` (+ _returnvalue (0.0 0.0 500.0)))
  (bind _outhit (`KismetSystemLibrary.LineTraceSingle` (`local.RayStart`) _rayend "TraceTypeQuery1" false (`local.ActorsToIgnore`) "ForDuration"))
  (bind (_bblockinghit _binitialoverlap _time _distance _location _impactpoint _normal _impactnormal) (`GameplayStatics.BreakHitResult` _outhit))
  (set `local.HitVector` (select `bool` _bblockinghit :`false` _rayend :`true` _location))
  (set `local.HitNormal` (select `bool` _bblockinghit :`false` (0.0 0.0 -1.0) :`true` _impactnormal))
  (`KismetSystemLibrary.DrawDebugBox` (+ (`local.HitVector`) (* _hitnormal _boxextent_x)) (`local.BoxExtent`) (struct :`R` 1.0 :`G` 1.0 :`B` 1.0 :`A` 1.0) _returnvalue_2)
  (`KismetSystemLibrary.DrawDebugPoint` _returnvalue_3 10.0 (struct :`R` 1.0 :`B` 0.477403 :`A` 1.0) 1.0)
  (return _returnvalue_3))

(fn `UserConstructionScript`)