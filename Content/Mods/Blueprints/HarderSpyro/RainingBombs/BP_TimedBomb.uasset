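; Timed bomb for the HarderSpyro mod's RainingBombs feature, which explodes on its own after a long delay.
; On BeginPlay it runs the parent logic, makes the player character its owner and starts a three-minute delay.
; When the delay ends it activates the Wick component and immediately forces the inherited Falcon level actor state machine into its Boom state.
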(event `self.ReceiveBeginPlay`
  (`parent.ReceiveBeginPlay`)
  (`self.SetOwner` (`GameplayStatics.GetPlayerCharacter` 0))
  (`KismetSystemLibrary.Delay` 180.0)
  (`ActorComponent.Activate` (`self.Wick`) false)
  (`FalconEnemyComponent.BP_ChangeState_StateComponent` (`self.FalconLevelActorStateMachine`) (`self.FalconLevelActorState_Boom`) true))

(fn `UserConstructionScript`
  (`parent.UserConstructionScript`))