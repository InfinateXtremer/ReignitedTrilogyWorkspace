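; Harder Spyro mod actor that makes Gnasty Gnorc's basic projectile kill the player in one hit.
; Tick binds to the player's damage delegate and the global transporter's level visibility event.
; A matching hit outside cutscenes applies a high-level damage effect, then swaps the character mesh for a frozen PoseableMesh copy of its pose.
; The normal mesh returns after a delay or when level visibility changes.
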(event `self.ReceiveTick`
  (params (DeltaSeconds :type "Float (single-precision)"))
  (bind _asbp_cps1999_playable (cast `/CPS1999_Spyro/Blueprints/BP_CPS1999_Playable` (`GameplayStatics.GetPlayerCharacter` 0)))
  (add `PhasmidCharacter.OnTakeDamageDelegate` _asbp_cps1999_playable (delegate `CustomEvent_0`))
  (bind _globaltransporter (`/GameplayCommon/LevelMechanics/LevelStreaming/Actors/TransportFunctions.FindGlobalTransporter`))
  (add `TransportManager.LevelVisibilityEvent` _globaltransporter (delegate `CustomEvent_1`)))

(event `CustomEvent_1`
  (params (LevelName :type Name) (visible :type Boolean))
  (`SceneComponent.SetHiddenInGame` (`self.PoseableMesh`) true false)
  (`SceneComponent.SetHiddenInGame` (`Character.Mesh` (`GameplayStatics.GetPlayerCharacter` 0)) false false))

(event `CustomEvent_0`
  (params (Actor :type "Actor Object Reference") (Payload :type "GameplayEventData Structure"))
  (bind _poseablemesh (`self.PoseableMesh`))
  (bind _mesh (`Character.Mesh` (`GameplayStatics.GetPlayerCharacter` 0)))
  ;[1 1 1] Make sure it's gnasty's projectile
  (if (`KismetStringLibrary.Contains` (`KismetSystemLibrary.GetDisplayName` (`.Instigator` (break `GameplayEventData` Payload))) "GnastyGnorc_BasicProjectile")
    (if (not (`BlueprintGameplayTagLibrary.HasAnyTags` (`GameplayTagAssetInterface.GetOwnedGameplayTags` (`AbilitySystemBlueprintLibrary.GetAbilitySystemComponent` (`GameplayStatics.GetPlayerCharacter` 0))) (`BlueprintGameplayTagLibrary.MakeLiteralGameplayTagContainer` (struct :`GameplayTags` (struct :`(TagName` "Character.Cutscene") :`(TagName` "Character.IsInLevelTransition") :`(TagName` "DamageSystem.Prevented.Invulnerable") :`(TagName` "DamageSystem.Prevented.DamageGroup"))))))
      (`AbilitySystemComponent.BP_ApplyGameplayEffectToSelf` :`self` (cast `PhasmidAbilitySystemComponent` (`AbilitySystemBlueprintLibrary.GetAbilitySystemComponent` (`GameplayStatics.GetPlayerCharacter` 0)) :!pure true) :`GameplayEffectClass` "/CharacterCommon/Abilities/GameplayEffects/GE_BasicDamage.GE_BasicDamage_C" :`Level` 5.0)
      (cast `/CPS1999_Spyro/Blueprints/BP_CPS1999_Playable` (`GameplayStatics.GetPlayerCharacter` 0))
      (`PoseableMeshComponent.CopyPoseFromSkeletalComponent` _poseablemesh _mesh)
      (`SceneComponent.K2_AttachToComponent` _poseablemesh _mesh "None" "SnapToTarget" "SnapToTarget" "SnapToTarget" true)
      (`SceneComponent.SetHiddenInGame` (`self.PoseableMesh`) false false)
      (`SceneComponent.SetHiddenInGame` (`Character.Mesh` (`GameplayStatics.GetPlayerCharacter` 0)) true false)
      (`KismetSystemLibrary.Delay` 4.0)
      (`SceneComponent.SetHiddenInGame` (`self.PoseableMesh`) true false)
      (`SceneComponent.SetHiddenInGame` (`Character.Mesh` (`GameplayStatics.GetPlayerCharacter` 0)) false false))))

(fn `UserConstructionScript`)