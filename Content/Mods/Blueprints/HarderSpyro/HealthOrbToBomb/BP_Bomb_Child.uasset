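; Child bomb for the HarderSpyro mod's HealthOrbToBomb feature that detonates itself after spawning.
; On BeginPlay it makes the player character its owner, then forces the level actor state machine into its Boom state.
; Unless Instant is set, it first lights the wick and waits a short delay drawn from a fixed-seed random stream, so the fuse time is effectively constant.
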(event `self.ReceiveBeginPlay`
  (`parent.ReceiveBeginPlay`)
  (`self.SetOwner` (`GameplayStatics.GetPlayerCharacter` 0))
  (if (not (`self.Instant`))
    (`ActorComponent.Activate` (`self.Wick`) false)
    (`KismetSystemLibrary.Delay` (`KismetMathLibrary.RandomFloatInRangeFromStream` 0.4 2.0 (`KismetMathLibrary.MakeRandomStream` 0))))
  (`FalconEnemyComponent.BP_ChangeState_StateComponent` (`self.FalconLevelActorStateMachine`) (`self.FalconLevelActorState_Boom`) true))

(fn `UserConstructionScript`
  (`parent.UserConstructionScript`))