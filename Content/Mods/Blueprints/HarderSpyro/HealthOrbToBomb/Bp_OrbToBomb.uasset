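; Harder-Spyro mod actor that turns health pickups into bombs (BP_Bomb_Child).
; Enemy drop lists are rebuilt to replace life orbs with bombs, or to roll bomb or orb by Percentage when Chance is set.
; Selected 1-Up chests lose their item or spawn a bomb on fracture, using a seed-0 random stream.
; Tick reapplies changes on level change, after player death, and until a SanityCheck counter reaches ten.
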(event `self.ReceiveBeginPlay`
  (bind _globaltransporter (`/GameplayCommon/LevelMechanics/LevelStreaming/Actors/TransportFunctions.FindGlobalTransporter`))
  (add `TransportManager.LoadCompleted` _globaltransporter (delegate `CustomEvent_1`)))

(event `CustomEvent_1`
  (bind _outactors (`GameplayStatics.GetAllActorsOfClass` "/CharacterCommon/BaseClasses/BP_Base_Enemy.BP_Base_Enemy_C" :!label _label))
  (for _array_element _outactors
    (for _array_element_2 (`self.K2_GetComponentsByClass` _array_element "/Script/Phasmid.FalconEnemyStateComponent")
      (bind _state (`FalconEnemyStateComponent.State` _array_element_2))
      (bind _newlocalvar_01 (`self.UpdateEnemyDrops` (`.SpawnCollectibles` (break `FalconEverythingState` _state))))
      (setmembers `FalconEverythingState` :`StructRef` _state :`SpawnCollectibles` _newlocalvar_01)))
  (bind _level_name (message `/GameplayCommon/GameModes/GameStateInterface.get current level name` (`GameplayStatics.GetGameState`)))
  (set `self.currentLevel` _level_name)
  (`/Engine/EditorBlueprintResources/StandardMacros.IncrementInt` (`self.SanityCheck`)))

(event `self.ReceiveTick`
  (params (DeltaSeconds :type "Float (single-precision)"))
  (bind _asbp_base_playable (cast `/CharacterCommon/BaseClasses/BP_Base_Playable` (`GameplayStatics.GetPlayerCharacter` 0)))
  (add `PhasmidCharacter.OnDeathDelegate` _asbp_base_playable (delegate `CustomEvent_0`))
  (bind _level_name (message `/GameplayCommon/GameModes/GameStateInterface.get current level name` (`GameplayStatics.GetGameState`)))
  (if (`KismetStringLibrary.NotEqual_StrStr` _level_name (`self.currentLevel`))
    (`self.HealthContainerToBomb` :!label _label_2)
    (goto _label)
    (elif (!= (`self.SanityCheck`) 10)
      (goto _label_2))))

(event `CustomEvent_0`
  (params (Actor :type "Actor Object Reference") (Payload :type "GameplayEventData Structure"))
  (`KismetSystemLibrary.Delay` 0.2)
  (set `self.currentLevel` ""))

(event `HealthContainerToBomb`
  ;[1 1 1] 1-Up Container To Bomb
  (bind _outactors (`GameplayStatics.GetAllActorsOfClass` "/GameplayCommon/LevelMechanics/TreasureChest/TreasureChest_Spyro1/BP_TreasureChest_1-Up.BP_TreasureChest_1-Up_C"))
  (for _array_element _outactors
    (bind _phasmidobjectsave (`/GameplayCommon/LevelMechanics/TreasureChest/TreasureChest_Assets/BP_TreasureChest_BASE.PhasmidObjectSave` _array_element))
    (bind _phasmidobjectsavedatalist (`self.UpdateCollectibleDrop` (`.saveDataList` (break `PhasmidObjectSaveDataList` (`PhasmidObjectSaveComponent.objectSaveData` _phasmidobjectsave)))))
    (set `PhasmidObjectSaveComponent.objectSaveData` _phasmidobjectsavedatalist _phasmidobjectsave)
    (if (`KismetMathLibrary.RandomBoolWithWeightFromStream` (`self.Percentage`) (`KismetMathLibrary.MakeRandomStream` 0))
      (add `DestructibleComponent.OnComponentFracture` (`/GameplayCommon/LevelMechanics/TreasureChest/TreasureChest_Assets/BP_TreasureChest_BASE.Destructible` _array_element) (delegate `CustomEvent_3`)))))

(event `CustomEvent_3`
  (params (HitPoint :type "Vector Structure (by ref)") (HitDirection :type "Vector Structure (by ref)"))
  ;[1 1 1] 1-Up Container To Bomb
  (`|SpawnActorFromClass` "/Game/Mods/Blueprints/HarderSpyro/HealthOrbToBomb/BP_Bomb_Child.BP_Bomb_Child_C" (`KismetMathLibrary.MakeTransform` (`self.K2_GetActorLocation` (stale `HealthContainerToBomb` _array_element))) "Undefined" "OverrideRootScale" null true null))

(fn `UpdateCollectibleDrop`
  (params (Array :type "Array of PhasmidObjectSaveData Structure"))
  (returns (PhasmidObjectSaveDataList :type "PhasmidObjectSaveDataList Structure"))
  (locals (NewLocalVar_1 :type "Array of PhasmidObjectSaveData Structure"))
  (for _array_element Array
    (bind (_itemdata _itemparamlist) (break `PhasmidObjectSaveData` _array_element))
    (`KismetArrayLibrary.Array_Add` (`local.NewLocalVar_1`) (select `bool` (`KismetMathLibrary.RandomBoolWithWeightFromStream` (`self.Percentage`) (`KismetMathLibrary.MakeRandomStream` 0)) :`false` _array_element :`true` (make `PhasmidObjectSaveData` (make `PhasmidInventoryData` "EIT_None" (`.collected` (break `PhasmidInventoryData` _itemdata))) _itemparamlist))))
  (return (make `PhasmidObjectSaveDataList` (`local.NewLocalVar_1`))))

(fn `UpdateEnemyDrops`
  (params (Array :type "Array of FalconEnemySpawnedCollectible Structure"))
  (returns (NewLocalVar_01 :type "Array of FalconEnemySpawnedCollectible Structure"))
  (locals (NewLocalVar_0 :type "Array of FalconEnemySpawnedCollectible Structure"))
  (bind _newlocalvar_0 (`local.NewLocalVar_0`))
  (for _array_element Array
    (bind (_collectibletype _alternatetype _collectible _bcollected) (break `FalconEnemySpawnedCollectible` _array_element))
    (`KismetArrayLibrary.Array_Add` _newlocalvar_0 (make `FalconEnemySpawnedCollectible` _collectibletype (select `bool` (`self.Chance?`) :`false` (select `bool` (== _alternatetype "/GameplayCommon/LevelMechanics/Loot/Loot_Spyro1/BP_S1_LifeOrb.BP_S1_LifeOrb_C") :`false` _alternatetype :`true` "/Game/Mods/Blueprints/HarderSpyro/HealthOrbToBomb/BP_Bomb_Child.BP_Bomb_Child_C") :`true` (select `bool` (`KismetMathLibrary.RandomBoolWithWeight` (`self.Percentage`)) :`false` "/GameplayCommon/LevelMechanics/Loot/Loot_Spyro1/BP_S1_LifeOrb.BP_S1_LifeOrb_C" :`true` "/Game/Mods/Blueprints/HarderSpyro/HealthOrbToBomb/BP_Bomb_Child.BP_Bomb_Child_C" :!type "PhasmidLevelActor Class Reference")) _collectible _bcollected)))
  (return _newlocalvar_0))

(fn `UserConstructionScript`)