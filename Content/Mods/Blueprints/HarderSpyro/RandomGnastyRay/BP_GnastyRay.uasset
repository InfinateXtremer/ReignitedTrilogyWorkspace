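; Harder Spyro mod actor that spawns a Gnasty Gnorc projectile from a randomly raycast point.
; On BeginPlay it casts repeated random upward traces from the player (itself outside packaged builds), then spawns the projectile at the chosen trace's end, aimed back at its start.
; CastRandomRay resets the longest distance each call, so the last valid trace wins, not the longest.
; Two debug keys spawn projectiles near world origin, using forward vector plus offset as location.
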(event `self.ReceiveBeginPlay`
  (bind (_bblockinghit _binitialoverlap _time _distance _location _impactpoint _normal _impactnormal _physmat _hitactor _hitcomponent _hitbonename _hititem _faceindex _tracestart _traceend) (`GameplayStatics.BreakHitResult` (`self.curHit`)))
  (for _ (range 21)
    (`self.CastRandomRay`))
  (`KismetSystemLibrary.PrintString` (`KismetStringLibrary.BuildString_Double` "" "LongestRay:" (`self.curLongestDistance`)))
  (`KismetSystemLibrary.DrawDebugLine` _tracestart _traceend (struct :`R` 1.0 :`B` 0.385523 :`A` 1.0) 3.0 10.0)
  (`|SpawnActorFromClass` "/CBS1005_GnastyGnorc/Blueprints/GnastyGnorc_BasicProjectile.GnastyGnorc_BasicProjectile_C" (`KismetMathLibrary.MakeTransform` _traceend (`KismetMathLibrary.FindLookAtRotation` _traceend _tracestart)) "Undefined" "OverrideRootScale" null null))

(event `CastRandomRay`
  (bind _returnvalue (`self.K2_GetActorLocation` (select `bool` (`KismetSystemLibrary.IsPackagedForDistribution`) :`false` self :`true` (`GameplayStatics.GetPlayerCharacter` 0) :!type "Actor Object Reference")))
  (set `self.curLongestDistance` 0.0)
  (set `self.curHit` (struct))
  (set `self.RayStart` _returnvalue)
  (set `self.RayEnd` (+ _returnvalue (* (`KismetMathLibrary.MakeVector` (`KismetMathLibrary.RandomFloatInRange` -1.0 1.0) (`KismetMathLibrary.RandomFloatInRange` -1.0 1.0) (`KismetMathLibrary.RandomFloatInRange` 0.2 1.0)) 10000.0)))
  (bind _outhit (`KismetSystemLibrary.LineTraceSingle` (`self.RayStart`) (`self.RayEnd`) "TraceTypeQuery1" true (`|MakeArray` (`GameplayStatics.GetPlayerPawn` 0) :!type "Actor Object Reference") "ForDuration"))
  (bind _returnvalue_2 (`KismetMathLibrary.VSize` (- (`.Location` (`GameplayStatics.BreakHitResult` _outhit)) (`self.RayStart`))))
  (if (> _returnvalue_2 (`self.curLongestDistance`))
    (set `self.curLongestDistance` _returnvalue_2)
    (set `self.curHit` _outhit)))

(event `Key|ü` :consume false :overrideparent false
  (params (Key :type "Key Structure"))
  (bind _returnvalue (+ (`self.GetActorForwardVector` (select `bool` (`KismetSystemLibrary.IsPackagedForDistribution`) :`false` self :`true` (`GameplayStatics.GetPlayerCharacter` 0) :!type "Actor Object Reference")) (100.0 0.0 50.0)))
  (:`Pressed`
    (`/Game/ModLoader/Blueprints/Widgets/Utility/BF_PrintText.BF_PrintString` "Trying to spawn ray" :!label _label)
    (`|SpawnActorFromClass` "/CBS1005_GnastyGnorc/Blueprints/GnastyGnorc_BasicProjectile.GnastyGnorc_BasicProjectile_C" (`KismetMathLibrary.MakeTransform` _returnvalue) "Undefined" "OverrideRootScale" null null)
    (`KismetSystemLibrary.DrawDebugSphere` _returnvalue 100.0 12 (struct :`R` 1.0 :`G` 1.0 :`B` 1.0 :`A` 1.0) 50.0)))

(event `Key|NumPadNine` :consume false :overrideparent false
  (params (Key :type "Key Structure"))
  (:`Pressed`
    (goto _label)))

(fn `UserConstructionScript`)