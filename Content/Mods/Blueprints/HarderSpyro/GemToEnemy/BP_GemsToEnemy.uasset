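; Harder Spyro mod actor that swaps level gems for random enemies.
; On level visibility changes (or BeginPlay when unpackaged), it removes previous spawns, restores gems, then reads the level's enemy classes from a data table.
; Gems passing a seeded Chance roll are sunk below ground, mapped to spawned enemies whose death-state collectibles are rewritten.
; Tick binds both delegates; damaging a mapped enemy moves its gem there and force-collects it.
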(event `self.ReceiveTick`
  (params (DeltaSeconds :type "Float (single-precision)"))
  (bind _globaltransporter (`/GameplayCommon/LevelMechanics/LevelStreaming/Actors/TransportFunctions.FindGlobalTransporter`))
  (add `TransportManager.LevelVisibilityEvent` _globaltransporter (delegate `CustomEvent_1`))
  (bind _keys (`BlueprintMapLibrary.Map_Keys` (`self.EnemyGemRelation`)))
  (for _array_element _keys
    (bind _asbp_base_enemy (cast `/CharacterCommon/BaseClasses/BP_Base_Enemy` _array_element))
    (add `PhasmidCharacter.OnTakeDamageDelegate` _asbp_base_enemy (delegate `CustomEvent_2`))))

(event `CustomEvent_2`
  (params (Actor :type "Actor Object Reference") (Payload :type "GameplayEventData Structure"))
  (bind (_value _returnvalue) (`BlueprintMapLibrary.Map_Find` (`self.EnemyGemRelation`) Actor))
  (`/Game/ModLoader/Blueprints/Widgets/Utility/BF_PrintText.BF_PrintString` "I'm dead")
  (`/Game/ModLoader/Blueprints/Widgets/Utility/BF_PrintText.BF_PrintString` (select `bool` _returnvalue :`false` "Cannot find the gem" :`true` "Found the gem that should be collected."))
  (`self.K2_SetActorLocation` _value (`self.K2_GetActorLocation` Actor) false false)
  (`KismetSystemLibrary.Delay` 0.1)
  (message `/GameplayCommon/LevelMechanics/Loot/Loot_Assets/LootInterface.ILootSetForceAutoCollect` _value true))

(event `self.ReceiveBeginPlay`
  (bind _gemvectorarray (`self.GemVectorArray`))
  (bind _currentlevel (`self.currentLevel`))
  (if (not (`KismetSystemLibrary.IsPackagedForDistribution`))
    (bind _returnvalue (`KismetStringLibrary.Conv_NameToString` (select `bool` (`KismetSystemLibrary.IsPackagedForDistribution`) :`false` "/LS101_ArtisansHome/Test" :`true` (stale `CustomEvent_1` LevelName))))
    (bind _returnvalue_2 (`KismetStringLibrary.GetSubstring` _returnvalue 1 (- (`KismetStringLibrary.FindSubstring` _returnvalue "/" false false 2) 1)))
    (`/Game/ModLoader/Blueprints/Widgets/Utility/BF_PrintText.BF_PrintString` (`KismetStringLibrary.Concat_StrStr` "Starting at: " _returnvalue_2) :!label _label)
    (bind _outactors (`GameplayStatics.GetAllActorsWithTag` (`KismetStringLibrary.Conv_StringToName` (`self.currentLevel`))))
    (for _array_element _outactors
      (`self.K2_DestroyActor` _array_element)
      (`/Game/ModLoader/Blueprints/Widgets/Utility/BF_PrintText.BF_PrintString` "Extra enemies removed.")
      ;[1 1 1] Restore gem location
      (bind _keys (`BlueprintMapLibrary.Map_Keys` _gemvectorarray))
      (for _array_element_2 _keys
        (`self.K2_SetActorLocation` (`|ConvertAsset` (`BlueprintMapLibrary.Map_Find` _gemvectorarray _array_element_2)) _array_element_2 false false))
      (`BlueprintMapLibrary.Map_Clear` (`self.GemVectorArray`)))
    (`BlueprintMapLibrary.Map_Clear` (`self.EnemyGemRelation`))
    (set `self.currentLevel` _returnvalue_2)
    (`/Game/ModLoader/Blueprints/Widgets/Utility/BF_PrintText.BF_PrintString` "Getting enemies from data table")
    ;[1 1 1] Get random enemies from data table
    (bind _returnvalue_3 (`|GetDataTableRow` "/Game/Mods/Blueprints/HarderSpyro/GemToEnemy/EnemyList.EnemyList" (`KismetStringLibrary.Conv_StringToName` _currentlevel))
      (:`then`
        (set `self.EnemyClasses` (`.EnemyList_5_F40DD9514EE567707DED10B5DFC2931B` (break `/Game/Mods/Blueprints/HarderSpyro/GemToEnemy/EnemyListStruct` _returnvalue_3)))
        (bind _gemclassarray1 (`self.CreateGemArray`))
        (`/Game/ModLoader/Blueprints/Widgets/Utility/BF_PrintText.BF_PrintString` (`KismetStringLibrary.BuildString_Int` "" "Gem Array Length: " (`KismetArrayLibrary.Array_Length` _gemclassarray1)))
        (for _array_element_3 _gemclassarray1
          (if (`KismetMathLibrary.RandomBoolWithWeightFromStream` (`self.Chance`) (`KismetMathLibrary.MakeRandomStream` 0))
            (`BlueprintMapLibrary.Map_Add` (`self.GemVectorArray`) (`self.K2_GetActorLocation` _array_element_3) (`|ConvertAsset` _array_element_3))
            (bind _returnvalue_4 (`self.K2_GetActorLocation` _array_element_3))
            (bind _returnvalue_5 (`self.HandleEnemySpawning` _returnvalue_4))
            (`self.HandleEnemyLoot` _returnvalue_5 _array_element_3)
            (`self.K2_SetActorLocation` _array_element_3 (+ _returnvalue_4 (0.0 0.0 -1000.0)) false false)
            (`BlueprintMapLibrary.Map_Add` (`self.EnemyGemRelation`) _returnvalue_5 _array_element_3))))
      (:`RowNotFound`
        (`/Game/ModLoader/Blueprints/Widgets/Utility/BF_PrintText.BF_PrintString` (`KismetStringLibrary.Concat_StrStr` "Row not found for the level: " _currentlevel))))))

(event `CustomEvent_1`
  (params (LevelName :type Name) (visible :type Boolean))
  (`KismetSystemLibrary.Delay` 0.1)
  (goto _label))

(fn `CreateGemArray`
  (returns (GemClassArray1 :type "Array of Actor Object Reference"))
  (locals (GemClassArray :type "Array of Actor Object Reference"))
  (bind _gemclassarray (`local.GemClassArray`))
  (bind _gemclassarray_2 (`local.GemClassArray`))
  (bind _outactors (`GameplayStatics.GetAllActorsOfClass` "/GameplayCommon/LevelMechanics/Loot/Loot_Spyro1/BP_S1_Gem_Blue.BP_S1_Gem_Blue_C"))
  (`KismetArrayLibrary.Array_Append` _gemclassarray_2 _outactors)
  (bind _outactors_2 (`GameplayStatics.GetAllActorsOfClass` "/GameplayCommon/LevelMechanics/Loot/Loot_Spyro1/BP_S1_Gem_Green.BP_S1_Gem_Green_C"))
  (`KismetArrayLibrary.Array_Append` _gemclassarray_2 _outactors_2)
  (bind _outactors_3 (`GameplayStatics.GetAllActorsOfClass` "/GameplayCommon/LevelMechanics/Loot/Loot_Spyro1/BP_S1_Gem_Purple.BP_S1_Gem_Purple_C"))
  (`KismetArrayLibrary.Array_Append` _gemclassarray_2 _outactors_3)
  (bind _outactors_4 (`GameplayStatics.GetAllActorsOfClass` "/GameplayCommon/LevelMechanics/Loot/Loot_Spyro1/BP_S1_Gem_Red.BP_S1_Gem_Red_C"))
  (`KismetArrayLibrary.Array_Append` _gemclassarray_2 _outactors_4)
  (bind _outactors_5 (`GameplayStatics.GetAllActorsOfClass` "/GameplayCommon/LevelMechanics/Loot/Loot_Spyro1/BP_S1_Gem_Yellow.BP_S1_Gem_Yellow_C"))
  (`KismetArrayLibrary.Array_Append` _gemclassarray_2 _outactors_5)
  (bind _outactors_6 (`GameplayStatics.GetAllActorsOfClass` "/GameplayCommon/LevelMechanics/Loot/Loot_Spyro2/BP_S2_Gem_Green.BP_S2_Gem_Green_C"))
  (`KismetArrayLibrary.Array_Append` _gemclassarray _outactors_6)
  (bind _outactors_7 (`GameplayStatics.GetAllActorsOfClass` "/GameplayCommon/LevelMechanics/Loot/Loot_Spyro2/BP_S2_Gem_Magenta.BP_S2_Gem_Magenta_C"))
  (`KismetArrayLibrary.Array_Append` _gemclassarray _outactors_7)
  (bind _outactors_8 (`GameplayStatics.GetAllActorsOfClass` "/GameplayCommon/LevelMechanics/Loot/Loot_Spyro2/BP_S2_Gem_Purple.BP_S2_Gem_Purple_C"))
  (`KismetArrayLibrary.Array_Append` _gemclassarray _outactors_8)
  (bind _outactors_9 (`GameplayStatics.GetAllActorsOfClass` "/GameplayCommon/LevelMechanics/Loot/Loot_Spyro2/BP_S2_Gem_Red.BP_S2_Gem_Red_C"))
  (`KismetArrayLibrary.Array_Append` _gemclassarray _outactors_9)
  (bind _outactors_10 (`GameplayStatics.GetAllActorsOfClass` "/GameplayCommon/LevelMechanics/Loot/Loot_Spyro2/BP_S2_Gem_Yellow.BP_S2_Gem_Yellow_C"))
  (`KismetArrayLibrary.Array_Append` _gemclassarray _outactors_10)
  (return (`local.GemClassArray`)))

(fn `GenerateEnemyArray`
  (params (Array :type "Array of Name"))
  (locals (EnemyClassList :type "Array of Actor Class Reference"))
  (bind _outactors (`GameplayStatics.GetAllActorsOfClass` "/CharacterCommon/BaseClasses/BP_Base_Enemy.BP_Base_Enemy_C"))
  (for _array_element _outactors
    _))

(fn `HandleEnemyLoot`
  (params (BP_Base_Enemy :type "Object Object Reference") (Bp_GemBase :type "Actor Object Reference"))
  (locals (NewLocalVar_0 :type "EInventoryType Enum" :default "EIT_YellowGem") (CollectibleArray :type "Array of FalconEnemySpawnedCollectible Structure") (GemBase :type "/GameplayCommon/LevelMechanics/Loot/Loot_Assets/BP_Gem_Base Object Reference"))
  (bind _returnvalue (`GameplayStatics.GetObjectClass` Bp_GemBase))
  (`|ExecutionSequence`
    (:`then_0`
      (castclass `/GameplayCommon/LevelMechanics/Loot/Loot_Spyro1/BP_S1_Gem_Blue` _returnvalue
        (:`then`
          (set `local.NewLocalVar_0` "EIT_BlueGem"))
        (:`CastFailed`
          (castclass `/GameplayCommon/LevelMechanics/Loot/Loot_Spyro1/BP_S1_Gem_Green` _returnvalue
            (:`then`
              (set `local.NewLocalVar_0` "EIT_GreenGem"))
            (:`CastFailed`
              (castclass `/GameplayCommon/LevelMechanics/Loot/Loot_Spyro1/BP_S1_Gem_Purple` _returnvalue
                (:`then`
                  (set `local.NewLocalVar_0` "EIT_PurpleGem"))
                (:`CastFailed`
                  (castclass `/GameplayCommon/LevelMechanics/Loot/Loot_Spyro1/BP_S1_Gem_Red` _returnvalue
                    (:`then`
                      (set `local.NewLocalVar_0` "EIT_RedGem"))
                    (:`CastFailed`
                      (castclass `/GameplayCommon/LevelMechanics/Loot/Loot_Spyro1/BP_S1_Gem_Yellow` _returnvalue
                        (:`then`
                          (set `local.NewLocalVar_0` "EIT_None"))
                        (:`CastFailed`
                          (castclass `/GameplayCommon/LevelMechanics/Loot/Loot_Spyro2/BP_S2_Gem_Green` null
                            (:`then`
                              (set `local.NewLocalVar_0` "EIT_S2GreenGem"))
                            (:`CastFailed`
                              (castclass `/GameplayCommon/LevelMechanics/Loot/Loot_Spyro2/BP_S2_Gem_Magenta` null
                                (:`then`
                                  (set `local.NewLocalVar_0` "EIT_S2MagentaGem"))
                                (:`CastFailed`
                                  (castclass `/GameplayCommon/LevelMechanics/Loot/Loot_Spyro2/BP_S2_Gem_Purple` null
                                    (:`then`
                                      (set `local.NewLocalVar_0` "EIT_S2PurpleGem"))
                                    (:`CastFailed`
                                      (castclass `/GameplayCommon/LevelMechanics/Loot/Loot_Spyro2/BP_S2_Gem_Yellow` null
                                        (:`then`
                                          (set `local.NewLocalVar_0` "EIT_S2YellowGem"))
                                        (:`CastFailed`
                                          (castclass `/GameplayCommon/LevelMechanics/Loot/Loot_Spyro2/BP_S2_Gem_Red` null)
                                          (set `local.NewLocalVar_0` "EIT_S2RedGem"))))))))))))))))))))
    (:`then_1`
      (bind _asbp_gem_base (cast `/GameplayCommon/LevelMechanics/Loot/Loot_Assets/BP_Gem_Base` Bp_GemBase))
      (bind _output_get (set `local.GemBase` _asbp_gem_base))
      (bind _asbp_base_enemy (cast `/CharacterCommon/BaseClasses/BP_Base_Enemy` BP_Base_Enemy))
      (for _array_element (`self.K2_GetComponentsByClass` _asbp_base_enemy "/Script/Phasmid.FalconEnemyStateComponent")
        (if (== _array_element (`/CharacterCommon/BaseClasses/BP_Base_Enemy.State: LaunchToDeath` _asbp_base_enemy))
          (`KismetArrayLibrary.Array_Add` (`local.CollectibleArray`) (make `FalconEnemySpawnedCollectible` null "/GameplayCommon/LevelMechanics/Loot/Loot_Spyro1/BP_S1_LifeOrb.BP_S1_LifeOrb_C" null (`/GameplayCommon/LevelMechanics/Loot/Loot_Assets/BP_Loot_BASE.collected` _output_get)))
          (setmembers `FalconEverythingState` :`StructRef` (`FalconEnemyStateComponent.State` _array_element) :`SpawnCollectibles` (`local.CollectibleArray`))
          (else
            (setmembers `FalconEverythingState` :`StructRef` (`FalconEnemyStateComponent.State` _array_element) :`SpawnCollectibles` (`|MakeArray` (struct) :!type "FalconEnemySpawnedCollectible Structure"))))))))

(fn `HandleEnemySpawning`
  (params (SpawnTransform_Location :type "Vector Structure"))
  (returns (ReturnValue :type "/CharacterCommon/BaseClasses/BP_Base_Enemy Object Reference"))
  (bind _enemyclasses (`self.EnemyClasses`))
  (bind _returnvalue (`|SpawnActorFromClass` (`|GetArrayItem` _enemyclasses (`KismetMathLibrary.RandomInteger` (`KismetArrayLibrary.Array_Length` _enemyclasses))) (`KismetMathLibrary.MakeTransform` SpawnTransform_Location) "Undefined" "OverrideRootScale" null null))
  (`KismetArrayLibrary.Array_Add` (`Actor.Tags` _returnvalue) (`KismetStringLibrary.Conv_StringToName` (`self.currentLevel`)))
  (bind _asbp_base_enemy (cast `/CharacterCommon/BaseClasses/BP_Base_Enemy` _returnvalue)
    (:`then`
      (return _asbp_base_enemy))
    (:`CastFailed`
      (`/Game/ModLoader/Blueprints/Widgets/Utility/BF_PrintText.BF_PrintString` "Spawned enemy cast to base enemy failed."))))

(fn `UserConstructionScript`)