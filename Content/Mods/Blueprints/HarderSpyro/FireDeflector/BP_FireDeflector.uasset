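; Fire deflector actor for the HarderSpyro mod that punishes the player when fire damage is prevented by invulnerability.
; Its DealtDamage event checks the instigator tags for both fire and invulnerable-prevented damage, then after a short delay applies lava knock-up damage to the player character.
; An AlreadyHurt flag, cleared after a brief cooldown, limits repeat hits.
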(event `/Game/Mods/Blueprints/HarderSpyro/DamageCatcher/BPI_DamageCatcher.DealtDamage`
  (params (Actor :type "Actor Object Reference") (DamageInformation :type "GameplayEventData Structure"))
  (bind (_eventtag _instigator _target _optionalobject _optionalobject2 _contexthandle _instigatortags) (break `GameplayEventData` DamageInformation))
  (if (not (`self.AlreadyHurt?`))
    (if (and (`BlueprintGameplayTagLibrary.HasTag` _instigatortags (struct :`TagName` "DamageSystem.Prevented.Invulnerable")) (`BlueprintGameplayTagLibrary.HasTag` _instigatortags (struct :`TagName` "Damage.Fire")))
      (`KismetSystemLibrary.Delay` 0.1)
      (set `self.AlreadyHurt?` true)
      (`/CharacterCommon/AbilitySystem/DamageLibrary.Falcon: ApplyDamage` null (`GameplayStatics.GetPlayerCharacter` 0) 1.0 (struct :`GameplayTags` (struct :`(TagName` "Damage.LavaKnockUp"))))
      (`KismetSystemLibrary.Delay` 1.0)
      (set `self.AlreadyHurt?` false))))

(fn `UserConstructionScript`)