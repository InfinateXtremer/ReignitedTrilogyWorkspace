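; Mod actor that gives every gem a random color from a palette, and destroys itself on BeginPlay if multiple copies exist.
; Each Tick it binds to the global transporter's level visibility event, which recolors all BP_Gem_Base actors after a short delay.
; Each gem gets or reuses a dynamic material, whose vector parameters receive progressively darker HSV shades of the chosen color, also printed as debug text.
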(event `self.ReceiveBeginPlay`
  (bind _outactors (`GameplayStatics.GetAllActorsOfClass` "BP_GemColorRandomizer_C"))
  (for (_ _array_index) _outactors
    (if (!= _array_index 0)
      (`self.K2_DestroyActor`))))

(event `self.ReceiveTick`
  (params (DeltaSeconds :type "Float (single-precision)"))
  (bind _globaltransporter (`/GameplayCommon/LevelMechanics/LevelStreaming/Actors/TransportFunctions.FindGlobalTransporter`))
  (add `TransportManager.LevelVisibilityEvent` _globaltransporter (delegate `CustomEvent_0`)))

(event `CustomEvent_0`
  (params (LevelName :type Name) (visible :type Boolean))
  (bind _colors (`self.Colors`))
  (`KismetSystemLibrary.Delay` 0.2)
  (bind _outactors (`GameplayStatics.GetAllActorsOfClass` "/Script/Engine.Actor"))
  (for _array_element _outactors
    (bind _asbp_gem_base (cast `/GameplayCommon/LevelMechanics/Loot/Loot_Assets/BP_Gem_Base` _array_element))
    (bind _gemmaterial (`self.GetGemMaterial` _asbp_gem_base))
    (bind _colorsetup1 (`self.GenerateGemColorParameters` (`KismetMathLibrary.Conv_ColorToLinearColor` (`|GetArrayItem` _colors (`KismetMathLibrary.RandomIntegerInRange` 0 (- (`KismetArrayLibrary.Array_Length` _colors) 1))))))
    (`self.UpdateGemColor` _colorsetup1 _gemmaterial)))

(fn `GenerateGemColorParameters`
  (params (NewColor :type "LinearColor Structure"))
  (returns (ColorSetup1 :type "Map of Name to LinearColor Structure"))
  (locals (ColorSetup :type "Map of Name to LinearColor Structure") (Color :type "LinearColor Structure"))
  (bind (_h _s _v _a) (`KismetMathLibrary.RGBToHSV` (`local.Color`)))
  (set `local.Color` NewColor)
  (bind _keys (`BlueprintMapLibrary.Map_Keys` (`local.ColorSetup`)))
  (for (_array_element _array_index) _keys
    (bind _returnvalue (`KismetMathLibrary.HSVToRGB` _h _s (* _v (select `int` _array_index :`0` 1.0 :`1` 0.49 :`2` 0.32 :`3` 0.29 :`4` 0.15 :!type "Float (single-precision)")) _a))
    (`KismetSystemLibrary.PrintText` (`KismetTextLibrary.Conv_NameToText` _array_element) true true _returnvalue)
    (`BlueprintMapLibrary.Map_Add` (`local.ColorSetup`) _array_element _returnvalue))
  (return (`local.ColorSetup`)))

(fn `GetGemMaterial`
  (params (Actor :type "Actor Object Reference"))
  (returns (GemMaterial :type "MaterialInstanceDynamic Object Reference"))
  (bind _asbp_gem_base (cast `/GameplayCommon/LevelMechanics/Loot/Loot_Assets/BP_Gem_Base` Actor))
  (bind _gemmesh (`/GameplayCommon/LevelMechanics/Loot/Loot_Assets/BP_Loot_BASE.GemMesh` _asbp_gem_base))
  (bind _returnvalue (`PrimitiveComponent.GetMaterial` _gemmesh 0))
  (bind _asmaterial_instance_dynamic (cast `MaterialInstanceDynamic` _returnvalue)
    (:`then`
      (return _asmaterial_instance_dynamic))
    (:`CastFailed`
      (bind _returnvalue_2 (`PrimitiveComponent.CreateDynamicMaterialInstance` _gemmesh 0 _returnvalue))
      (return _returnvalue_2))))

(fn `UpdateGemColor`
  (params (TargetMap :type "Map of Name to LinearColor Structure (by ref)") (Material :type "MaterialInstanceDynamic Object Reference"))
  (bind _keys (`BlueprintMapLibrary.Map_Keys` TargetMap))
  (for _array_element _keys
    (bind (_value _returnvalue) (`BlueprintMapLibrary.Map_Find` TargetMap _array_element))
    (if _returnvalue
      (`MaterialInstanceDynamic.SetVectorParameterValue` Material _array_element _value))))

(fn `UserConstructionScript`)