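; Mod actor that randomizes where every PortalTransporter in the world leads when play begins.
; Each portal independently gets a level from shuffled Spyro1_StreamData row names, so destinations can repeat, and the pick is printed.
; It rewrites the portal's partner names to the level's "_LevelStart" and repoints its stream table row handles.
; The portal's name text is rebuilt from the display name found through SpyroStreamData and LevelMapTable2.
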(event `self.ReceiveBeginPlay`
  (bind _outactors (`GameplayStatics.GetAllActorsOfClass` "/GameplayCommon/LevelMechanics/LevelStreaming/Actors/PortalTransporter.PortalTransporter_C"))
  (for _array_element _outactors
    (bind _pickedlevel1 (`self.PickARandomLevel`))
    (`KismetSystemLibrary.PrintString` (`KismetStringLibrary.Conv_NameToString` _pickedlevel1))
    (`self.ChangePortalDestination` _array_element _pickedlevel1)))

(fn `ChangePortalDestination`
  (params (Object :type "Actor Object Reference") (InName :type Name))
  (locals (Levelname :type Name))
  (bind _returnvalue (`KismetStringLibrary.Concat_StrStr` (`KismetStringLibrary.Conv_NameToString` (`local.Levelname`)) "_LevelStart"))
  (set `local.Levelname` InName)
  (bind _asportal_transporter (cast `/GameplayCommon/LevelMechanics/LevelStreaming/Actors/PortalTransporter` Object))
  (set `Portal.PartnerPortalName` _returnvalue _asportal_transporter)
  (set `/GameplayCommon/LevelMechanics/LevelStreaming/Actors/BasePortal.PartnerPortalName_BASE` _returnvalue _asportal_transporter)
  (set `/GameplayCommon/LevelMechanics/LevelStreaming/Actors/BasePortal.LevelStreamTableRow` (make `DataTableRowHandle` "/GameplayCommon/LevelMechanics/LevelStreaming/StreamingData/LevelStreams/Spyro1_StreamData.Spyro1_StreamData" (`local.Levelname`)) _asportal_transporter)
  (set `Portal.PartnerPortalRow` (make `DataTableRowHandle` "/GameplayCommon/LevelMechanics/LevelStreaming/StreamingData/LevelStreams/SpyroStreamData.SpyroStreamData" (`local.Levelname`)) _asportal_transporter)
  (bind _returnvalue_2 (`|GetDataTableRow` "/GameplayCommon/LevelMechanics/LevelStreaming/StreamingData/LevelStreams/SpyroStreamData.SpyroStreamData" (`local.Levelname`))
    (:`then`
      (bind _returnvalue_3 (`|GetDataTableRow` "/GameplayCommon/LevelMechanics/LevelStreaming/StreamingData/LevelPaths/LevelMapTable2.LevelMapTable2" (`.LevelMapPath` (break `MasterLevelData` _returnvalue_2)))
        (:`then`
          (bind _portalnamecomponent (`/GameplayCommon/LevelMechanics/LevelStreaming/Actors/BasePortal.PortalNameComponent` _asportal_transporter))
          (`/GameplayCommon/LevelMechanics/LevelStreaming/Components/PortalNameComponent.REMAKE text` _portalnamecomponent (`.displayName_10_C5197E814C6E252831AEB18AA91091F8` (break `/GameplayCommon/LevelMechanics/LevelStreaming/StreamingData/LevelPaths/LevelInfoStruct` _returnvalue_3)) (`/GameplayCommon/LevelMechanics/LevelStreaming/Components/PortalNameComponent.Scale` _portalnamecomponent) (`/GameplayCommon/LevelMechanics/LevelStreaming/Components/PortalNameComponent.default char width` _portalnamecomponent)))))))

(fn `PickARandomLevel`
  (returns (PickedLevel1 :type Name))
  (locals (PickedLevel :type Name))
  (bind _outrownames (`DataTableFunctionLibrary.GetDataTableRowNames` "/GameplayCommon/LevelMechanics/LevelStreaming/StreamingData/LevelStreams/Spyro1_StreamData.Spyro1_StreamData"))
  (`KismetArrayLibrary.Array_Shuffle` _outrownames)
  (bind _output_get (set `local.PickedLevel` (`|GetArrayItem` _outrownames)))
  (return _output_get))

(fn `UserConstructionScript`)