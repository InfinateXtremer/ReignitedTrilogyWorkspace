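; BP_FlameLightColor is a mod manager actor that recolors the lights of fire attack effects.
; On BeginPlay it destroys itself if another instance is found first, acting as a singleton.
; Every tick it finds all FireAttackActorTrace actors and applies FlameColor to their spot and point lights.
; IChangeFlameColor updates that color; a non-zero color check exists but is disconnected.
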(event `self.ReceiveBeginPlay`
  (bind _outactors (`GameplayStatics.GetAllActorsOfClass` "BP_FlameLightColor_C"))
  (bind _output (`|GetArrayItem` _outactors))
  (if (and (`KismetSystemLibrary.IsValid` _output) (not (== _output self)))
    (`self.K2_DestroyActor`)))

(event `self.ReceiveTick`
  (params (DeltaSeconds :type "Float (single-precision)"))
  (bind _outactors (`GameplayStatics.GetAllActorsOfClass` "/CharacterCommon/Actors/FireAttack/FireAttackActorTrace.FireAttackActorTrace_C"))
  (for _array_element _outactors
    (`LightComponent.SetLightColor` (`SpyroFlameBreathActor.SpotLight` _array_element) (`self.FlameColor`) true)
    (`LightComponent.SetLightColor` (`SpyroFlameBreathActor.PointLightComp` _array_element) (`self.FlameColor`) true)))

(event `/Game/ModLoader/Blueprints/BPI_ModLoader.IChangeFlameColor`
  (params (NewColor :type "LinearColor Structure"))
  (set `self.FlameColor` NewColor))

(fn `UserConstructionScript`)