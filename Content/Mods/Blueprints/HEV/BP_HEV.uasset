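; HEV suit voice announcer that speaks warning lines when the player takes damage or dies.
; Tick binds the player's damage and death delegates; gameplay tags select heat, shock, flatten or poison lines, while Sparx health changes are only printed.
; HEVSpeak splits lines into tokens, plays each one's Sentences DataTable sound sequentially via audio-finished callbacks, and skips missing rows.
; Inline "(pNNN)" prefixes set per-token pitch as a percentage.
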(event `/CharacterCommon/Interfaces/ISparxActions.INotifySparxHealthChanged`
  (params (NewHealth :type "Float (single-precision)") (SkipReaction :type Boolean))
  (set `self.SparkHealth` NewHealth)
  (`/Game/ModLoader/Blueprints/Widgets/Utility/Macro_PrintText.Macro_PrintString` (`KismetStringLibrary.Concat_StrStr` "Sparx's Health Changed To: " (`KismetStringLibrary.Conv_DoubleToString` NewHealth)) (struct :`G` 0.665387 :`B` 1.0 :`A` 1.0) 1.0))

(event `OnDeathDelegate_Event_0`
  (params (Actor :type "Actor Object Reference") (Payload :type "GameplayEventData Structure"))
  (`self.HEVSpeak` (`self.GetRandomStringFromArray` (`self.Death`))))

(event `self.ReceiveTick`
  (params (DeltaSeconds :type "Float (single-precision)"))
  (bind _asbp_cps1999_playable (cast `/CPS1999_Spyro/Blueprints/BP_CPS1999_Playable` (`GameplayStatics.GetPlayerCharacter` 0)))
  (add `PhasmidCharacter.OnTakeDamageDelegate` _asbp_cps1999_playable (delegate `OnTakeDamageDelegate_Event_0`))
  (add `PhasmidCharacter.OnDeathDelegate` _asbp_cps1999_playable (delegate `OnDeathDelegate_Event_0`)))

(event `OnTakeDamageDelegate_Event_0`
  (params (Actor :type "Actor Object Reference") (Payload :type "GameplayEventData Structure"))
  (bind (_eventtag _instigator _target _optionalobject _optionalobject2 _contexthandle _instigatortags _targettags) (break `GameplayEventData` Payload))
  (`/Game/ModLoader/Blueprints/Widgets/Utility/BF_PrintText.BF_PrintString` (`KismetTextLibrary.Conv_TextToString` (`|FormatText` "TookDamage \n \nActor: {actor} \nInstigator: {instigator} \nContext Handle:{context} \nEvent Tag: {eventtag} \nInstigator Tags: {instigatortags} \nTarget Tags: {targettags} \nTarget Data: {targetdata} \n" (`KismetTextLibrary.Conv_StringToText` (`KismetSystemLibrary.GetDisplayName` _target)) (`KismetTextLibrary.Conv_StringToText` (`KismetSystemLibrary.GetDisplayName` _instigator)) (`KismetTextLibrary.Conv_StringToText` (`KismetSystemLibrary.GetDisplayName` (`AbilitySystemBlueprintLibrary.EffectContextGetSourceObject` _contexthandle))) (`KismetTextLibrary.Conv_NameToText` (`BlueprintGameplayTagLibrary.GetTagName` _eventtag)) (`KismetTextLibrary.Conv_StringToText` (`BlueprintGameplayTagLibrary.GetDebugStringFromGameplayTagContainer` _instigatortags)) (`KismetTextLibrary.Conv_StringToText` (`BlueprintGameplayTagLibrary.GetDebugStringFromGameplayTagContainer` _targettags)) _)))
  (if (`BlueprintGameplayTagLibrary.HasAnyTags` _instigatortags (`BlueprintGameplayTagLibrary.MakeLiteralGameplayTagContainer` (struct :`GameplayTags` (struct :`(TagName` "Damage.LavaKnockUp") :`(TagName` "Damage.World.LavaKnockUp") :`(TagName` "Damage.World.Lava")))))
    (`self.HEVSpeak` (`self.Heat`))
    (elif (`BlueprintGameplayTagLibrary.HasAnyTags` _instigatortags (`BlueprintGameplayTagLibrary.MakeLiteralGameplayTagContainer` (struct :`GameplayTags` (struct :`(TagName` "Damage.World.ZapKnockUp") :`(TagName` "Damage.Zap") :`(TagName` "Damage.ZapLong")))))
      (`self.HEVSpeak` "beep comma beep comma warning comma shock_damage")
      (elif (`BlueprintGameplayTagLibrary.HasAnyTags` _instigatortags (`BlueprintGameplayTagLibrary.MakeLiteralGameplayTagContainer` (struct :`GameplayTags` (struct :`(TagName` "Damage.Flatten") :`(TagName` "Damage.FlattenShort") :`(TagName` "Damage.HeadBash") :`(TagName` "Damage.KnockBack") :`(TagName` "Damage.KnockBackflip") :`(TagName` "Damage.KnockBackLong") :`(TagName` "Damage.KnockBackQuick") :`(TagName` "Damage.KnockBackShort") :`(TagName` "Damage.KnockSide.Left") :`(TagName` "Damage.KnockSide.Right") :`(TagName` "Damage.SgtByrd.Rocket.Blast") :`(TagName` "Damage.SgtByrd.Rocket.Impact") :`(TagName` "Damage.Simple") :`(TagName` "Damage.Slap") :`(TagName` "Damage.SlideBack") :`(TagName` "Damage.Special.Barrel") :`(TagName` "Damage.Tornado") :`(TagName` "Damage.Turret") :`(TagName` "Damage.Bullet") :`(TagName` "Damage.BounceWithRecovery") :`(TagName` "Damage.BounceBack") :`(TagName` "Damage.BossKnockUp") :`(TagName` "Damage.Bomb") :`(TagName` "Damage.Backflip")))))
        (`self.HEVSpeak` (`self.GetRandomStringFromArray` (`self.MiscDamage`)))
        (elif (`BlueprintGameplayTagLibrary.HasAnyTags` _instigatortags (`BlueprintGameplayTagLibrary.MakeLiteralGameplayTagContainer` (struct :`GameplayTags` (struct :`(TagName` "Damage.World.Poison")))))
          (`self.HEVSpeak` "(p160)boop comma (p160)boop comma (p160)boop comma blood_toxins"))))))

(event `self.ReceiveBeginPlay`
  (if (not (`KismetSystemLibrary.IsPackagedForDistribution`))
    (`self.HEVSpeak` "(p120)beep comma (p120)beep comma warning comma heat_damage")))

(event `Speak`
  (bind _returnvalue (`KismetStringLibrary.ParseIntoArray` (stale `HEVSpeak` Line)))
  (bind _output (`|GetArrayItem` _returnvalue (`self.i`)))
  (bind _returnvalue_2 (+ (`KismetStringLibrary.FindSubstring` _output ")" false true) 1))
  (bind _returnvalue_3 (not (and (`KismetStringLibrary.Contains` _output "(p") (`KismetStringLibrary.Contains` _output ")" false true))))
  (bind _returnvalue_4 (select `bool` _returnvalue_3 :`false` (`KismetStringLibrary.GetSubstring` _output _returnvalue_2 (- (`KismetStringLibrary.Len` _output) _returnvalue_2)) :`true` _output))
  (`KismetSystemLibrary.PrintString` _returnvalue_4 :!label _label)
  (bind _returnvalue_5 (`self.PitchDetection` _output _returnvalue_3))
  (`KismetSystemLibrary.PrintString` (`KismetStringLibrary.Conv_DoubleToString` _returnvalue_5))
  (bind _returnvalue_6 (`|GetDataTableRow` "/Game/Mods/Blueprints/HEV/Sentences.Sentences" (`KismetStringLibrary.Conv_StringToName` _returnvalue_4))
    (:`then`
      (bind _returnvalue_7 (`GameplayStatics.SpawnSound2D` (`.audio_6_7FD552DB40829DE4A16860900E12B0E5` (break `/Game/Mods/Blueprints/HEV/HEV_Sentences` _returnvalue_6)) 1.0 _returnvalue_5))
      (add `AudioComponent.OnAudioFinished` _returnvalue_7 (delegate `Skip`)))
    (:`RowNotFound`
      (`/Engine/EditorBlueprintResources/StandardMacros.IncrementInt` (`self.i`) :!label _label_2
        (:`  `
          (if (!= (`KismetArrayLibrary.Array_Length` _returnvalue) (`self.i`))
            (`self.Speak`)
            (else
              (set `self.i` 0)
              (`KismetSystemLibrary.PrintString` "Finished Speaking"))))))))

(event `HEVSpeak`
  (params (Line :type String))
  (set `self.i` 0)
  (goto _label))

(event `Skip`
  (goto _label_2))

(fn `UserConstructionScript`)