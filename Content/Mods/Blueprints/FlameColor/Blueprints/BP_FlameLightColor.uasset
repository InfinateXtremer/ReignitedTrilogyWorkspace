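; BP_FlameLightColor is a mod actor that recolors the lights on the game's fire attack trace actor.
; Every tick, it sets each light component on the cached FireActorTrace to the LightColor variable.
; While that reference is invalid, it scans all actors in the world for a display name containing "FireAttackActorTrace" and caches the match.
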(event `self.ReceiveTick`
  (params (DeltaSeconds :type "Float (single-precision)"))
  (`/Engine/EditorBlueprintResources/StandardMacros.IsValid` (`self.FireActorTrace`)
    (:`Is Valid`
      (for _array_element (`self.K2_GetComponentsByClass` (`self.FireActorTrace`) "/Script/Engine.LightComponent")
        (`LightComponent.SetLightColor` _array_element (`self.LightColor`) true)))
    (:`Is Not Valid`
      (bind _outactors (`GameplayStatics.GetAllActorsOfClass` "/Script/Engine.Actor"))
      (for _array_element_2 _outactors
        (if (`KismetStringLibrary.Contains` (`KismetSystemLibrary.GetDisplayName` _array_element_2) "FireAttackActorTrace")
          (set `self.FireActorTrace` _array_element_2))))))

(fn `UserConstructionScript`)