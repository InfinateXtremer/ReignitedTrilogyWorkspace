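; BP_HealthToMat is a mod actor that mirrors Sparx's health into a material parameter collection so materials can react to it.
; BeginPlay destroys the actor if another instance comes first in the world.
; Tick scans the player character's child actors for Sparx and writes health as HealthFloat and a per-level HealthColor to MPC_Utility_Values, with a debug print.
; The health-change event only prints, and damage interface functions are stubs returning false.
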(event `self.ReceiveBeginPlay`
  (bind _outactors (`GameplayStatics.GetAllActorsOfClass` "BP_HealthToMat_C"))
  (bind _output (`|GetArrayItem` _outactors))
  (if (and (`KismetSystemLibrary.IsValid` _output) (not (== _output self)))
    (`self.K2_DestroyActor`)))

(event `self.ReceiveTick`
  (params (DeltaSeconds :type "Float (single-precision)"))
  (for _array_element (`self.GetAllChildActors` (`GameplayStatics.GetPlayerCharacter` 0) true)
    (bind _asbp_cps1194_sparx (cast `/CPS1194_SparxNew/Blueprints/BP_CPS1194_Sparx` _array_element))
    (bind _cursparxhealth (`/CPS1194_SparxNew/Blueprints/BP_CPS1194_Sparx.CurSparxHealth` _asbp_cps1194_sparx))
    (`KismetMaterialLibrary.SetScalarParameterValue` "/Game/Mods/Blueprints/HealthToMaterial/MPC_Utility_Values.MPC_Utility_Values" "HealthFloat" (`KismetMathLibrary.Conv_IntToDouble` _cursparxhealth))
    (`/Game/ModLoader/Blueprints/Widgets/Utility/Macro_PrintText.Macro_PrintString` (`KismetStringLibrary.Concat_StrStr` "My current health is: " (`KismetStringLibrary.Conv_IntToString` _cursparxhealth)) (struct :`G` 0.665387 :`B` 1.0 :`A` 1.0) 1.0)
    (`KismetMaterialLibrary.SetVectorParameterValue` "/Game/Mods/Blueprints/HealthToMaterial/MPC_Utility_Values.MPC_Utility_Values" "HealthColor" (select `int` _cursparxhealth :`0` (struct :`A` 1.0) :`1` (struct :`R` 1.0 :`A` 1.0) :`2` (struct :`R` 0.226966 :`G` 1.0 :`A` 1.0) :`3` (struct :`G` 0.723055 :`B` 1.0 :`A` 1.0) :`4` (struct :`R` 1.0 :`G` 0.783538 :`A` 1.0) :!type "LinearColor Structure"))))

(event `/CharacterCommon/Interfaces/ISparxActions.INotifySparxHealthChanged`
  (params (NewHealth :type "Float (single-precision)") (SkipReaction :type Boolean))
  (`/Game/ModLoader/Blueprints/Widgets/Utility/Macro_PrintText.Macro_PrintString` (`KismetStringLibrary.Concat_StrStr` "Sparx's Health Changed To: " (`KismetStringLibrary.Conv_DoubleToString` NewHealth)) (struct :`G` 0.665387 :`B` 1.0 :`A` 1.0) 1.0))

(fn `IsChargeTarget`
  (returns (ReturnValue :type Boolean))
  (return false))

(fn `IsDead`
  (returns (ReturnValue :type Boolean))
  (return false))

(fn `IsImmuneToDamage`
  (params (InTagContainer :type "GameplayTagContainer Structure (by ref)") (HitComponent :type "PrimitiveComponent Object Reference"))
  (returns (ReturnValue :type Boolean))
  (return false))

(fn `OnDamage`
  (params (Payload :type "GameplayEventData Structure"))
  (returns (ReturnValue :type Boolean))
  (return false))

(fn `OnDealDamage`
  (params (Payload :type "GameplayEventData Structure"))
  (returns (ReturnValue :type Boolean))
  (return false))

(fn `OnDeath`
  (params (Payload :type "GameplayEventData Structure"))
  (returns (ReturnValue :type Boolean))
  (return false))

(fn `OnHealthRestored`
  (params (Payload :type "GameplayEventData Structure"))
  (returns (ReturnValue :type Boolean))
  (return false))

(fn `OnShieldBreak`
  (params (Payload :type "GameplayEventData Structure"))
  (returns (ReturnValue :type Boolean))
  (return false))

(fn `UserConstructionScript`)