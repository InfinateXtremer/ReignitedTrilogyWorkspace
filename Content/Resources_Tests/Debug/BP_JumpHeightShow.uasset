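; Debug test actor that measures the player's maximum jump height at a configured frame rate.
; While the player overlaps its Box, Tick caps the engine frame rate to FPS through a t.maxfps console command and tracks the highest player Z above the box.
; A text render shows the FPS setting and the running maximum.
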(event `self.ReceiveBeginPlay`
  (`TextRenderComponent.K2_SetText` (`self.TextRender`) (`|FormatText` "FPS: {fps}" (`self.FPS`))))

(event `self.ReceiveTick`
  (params (DeltaSeconds :type "Float (single-precision)"))
  (bind (_returnvalue_x _returnvalue_y _returnvalue_z) (`KismetMathLibrary.BreakVector` (`self.K2_GetActorLocation` (`GameplayStatics.GetPlayerCharacter` 0))))
  (bind (_returnvalue_x_2 _returnvalue_y_2 _returnvalue_z_2) (`KismetMathLibrary.BreakVector` (`SceneComponent.K2_GetComponentLocation` (`self.Box`))))
  (if (`PrimitiveComponent.IsOverlappingActor` (`self.Box`) (`GameplayStatics.GetPlayerCharacter` 0))
    (`KismetSystemLibrary.ExecuteConsoleCommand` (`KismetStringLibrary.Concat_StrStr` "t.maxfps " (`KismetStringLibrary.Conv_IntToString` (`self.FPS`))))
    (bind _output_get (set `self.MaxJumpHeight` (`KismetMathLibrary.FMax` (- _returnvalue_z _returnvalue_z_2) (`self.MaxJumpHeight`))))
    (`TextRenderComponent.K2_SetText` (`self.TextRender`) (`|FormatText` "FPS: {fps} - Max Jump Height: {height}" (`self.FPS`) _output_get))))

(fn `UserConstructionScript`)