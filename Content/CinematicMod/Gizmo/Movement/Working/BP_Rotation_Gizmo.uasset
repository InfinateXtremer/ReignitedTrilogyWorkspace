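; Rotation gizmo actor that lets the player rotate a target component by click-dragging X, Y or Z rings, in world or local space.
; Picks and highlights rings by intersecting the mouse ray with each axis plane and testing scaled ring radius.
; While dragging, applies the angle from the clicked point to the starting rotations and disables mesh physics, restoring it on release.
; When idle, it follows the target's location.
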(event `self.ReceiveBeginPlay`
  (`parent.ReceiveBeginPlay`)
  (`self.K2_SetActorRotation` (`KismetMathLibrary.ComposeRotators` (`SceneComponent.K2_GetComponentRotation` (`self.TargetComponent`)) (`KismetMathLibrary.RotatorFromAxisAndAngle` (`self.CurrentAxis`) (`/Game/CinematicMod/Utilities/CineMacroLibrary.GetAroundAxisBetweenTwoVector` (`self.FirstClickedPoint`) (`.IntersectionPoint` (`self.PlaneMath` (`self.CurrentAxis`))) (`self.CurrentAxis`))))))

(event `self.ReceiveTick`
  (params (DeltaSeconds :type "Float (single-precision)"))
  (bind _returnvalue (`KismetMathLibrary.RotatorFromAxisAndAngle` (`self.CurrentAxis`) (`/Game/CinematicMod/Utilities/CineMacroLibrary.GetAroundAxisBetweenTwoVector` (`self.FirstClickedPoint`) (`.IntersectionPoint` (`self.PlaneMath` (`self.CurrentAxis`))) (`self.CurrentAxis`))))
  (`self.HighlightAxis`)
  (`self.CalculateCameraDistanceFromGizmo`)
  (if (`self.Clicking`)
    (`self.K2_SetActorRotation` (`KismetMathLibrary.ComposeRotators` (`self.FirstRotation`) _returnvalue))
    (`SceneComponent.K2_SetWorldRotation` (`self.TargetComponent`) (`KismetMathLibrary.ComposeRotators` (`self.AttachedActorsRotation`) _returnvalue) false false)
    (bind _asmesh_component (cast `MeshComponent` (`self.TargetComponent`)))
    (`PrimitiveComponent.SetSimulatePhysics` _asmesh_component false)
    (else
      (`self.K2_SetActorLocation` (`SceneComponent.K2_GetComponentLocation` (`self.TargetComponent`))))))

(event `Key|LeftMouseButton` :consume false :overrideparent false
  (params (Key :type "Key Structure"))
  (:`Pressed`
    (bind (_ishoveringaxis _closestaxis1 _clickedpoint1) (`self.SelectAxis`))
    (if _ishoveringaxis
      (set `self.CurrentAxis` (`KismetMathLibrary.GreaterGreater_VectorRotator` (select `/Game/CinematicMod/Gizmo/Movement/Axis` _closestaxis1 :`NewEnumerator0` (1.0 0.0 0.0) :`NewEnumerator1` (0.0 1.0 0.0) :`NewEnumerator2` (0.0 0.0 1.0) :!type "Vector Structure") (`self.GetRotationSpace`)))
      (set `self.FirstClickedPoint` _clickedpoint1)
      (set `self.FirstRotation` (`self.K2_GetActorRotation`))
      (set `self.AttachedActorsRotation` (`SceneComponent.K2_GetComponentRotation` (`self.TargetComponent`)))
      (set `self.Clicking` true)
      (`/Engine/EditorBlueprintResources/StandardMacros.DoOnce` false :!label _label
        (:`Completed`
          (set `self.WasSimulatingPhysics` (`SceneComponent.IsSimulatingPhysics` (`self.TargetComponent`) "None"))))))
  (:`Released`
    (set `self.Clicking` false)
    (`self.K2_SetActorRotation` (`self.GetRotationSpace`))
    (bind _asmesh_component (cast `MeshComponent` (`self.TargetComponent`)))
    (`PrimitiveComponent.SetSimulatePhysics` _asmesh_component (`self.WasSimulatingPhysics`))
    (goto _label :!via `Reset`)))

(fn `Debug`
  (params (Center :type "Vector Structure") (LineColor :type "LinearColor Structure") (Distance :type "Float (double-precision)")))

(fn `HighlightAxis`
  (bind (_ishoveringaxis _closestaxis1) (`self.SelectAxis`))
  (if (and _ishoveringaxis (not (`self.Clicking`)))
    (`self.SetMaterialValue` (select `/Game/CinematicMod/Gizmo/Movement/Axis` _closestaxis1 :`NewEnumerator0` (`self.X`) :`NewEnumerator1` (`self.Y`) :`NewEnumerator2` (`self.Z`) :!type "Object Object Reference") 1.0)
    (else
      (`self.SetMaterialValue` (`self.Y`))
      (`self.SetMaterialValue` (`self.Z`))
      (`self.SetMaterialValue` (`self.X`)))))

(fn `SelectAxis`
  (returns (IsHoveringAxis :type Boolean) (ClosestAxis1 :type "/Game/CinematicMod/Gizmo/Movement/Axis Enum") (ClickedPoint1 :type "Vector Structure"))
  (locals (ClosestDistance :type "Float (double-precision)" :default 1.0) (ClosestAxis :type "/Game/CinematicMod/Gizmo/Movement/Axis Enum") (ClickedPoint :type "Vector Structure"))
  (bind (_returnvalue _t _intersectionpoint) (`self.CalculateIfAxisIsUnderTheMouse` "NewEnumerator0" (`local.ClosestDistance`)))
  (bind (_returnvalue_2 _t_2 _intersectionpoint_2) (`self.CalculateIfAxisIsUnderTheMouse` "NewEnumerator1" (`local.ClosestDistance`)))
  (bind (_returnvalue_3 _t_3 _intersectionpoint_3) (`self.CalculateIfAxisIsUnderTheMouse` "NewEnumerator2" (`local.ClosestDistance`)))
  (set `local.ClosestDistance` 1.0)
  (`|ExecutionSequence`
    (:`then_0`
      (if _returnvalue
        (set `local.ClosestDistance` _t)
        (set `local.ClickedPoint` _intersectionpoint)
        (set `local.ClosestAxis` "NewEnumerator0")))
    (:`then_1`
      (if _returnvalue_2
        (set `local.ClosestDistance` _t_2)
        (set `local.ClickedPoint` _intersectionpoint_2)
        (set `local.ClosestAxis` "NewEnumerator1")))
    (:`then_2`
      (if _returnvalue_3
        (set `local.ClosestDistance` _t_3)
        (set `local.ClickedPoint` _intersectionpoint_3)
        (set `local.ClosestAxis` "NewEnumerator2")))
    (:`then_3`
      (return (< (`local.ClosestDistance`) 1.0) (`local.ClosestAxis`) (`local.ClickedPoint`)))))

(fn `SetCurrentLocationAndOffset`)

(fn `SetMaterialValue`
  (params (Object :type "Object Object Reference") (Value :type "Float (double-precision)"))
  (locals (meshcomp :type "StaticMeshComponent Object Reference") (material :type "MaterialInstanceDynamic Object Reference"))
  (bind _asstatic_mesh_component (cast `StaticMeshComponent` Object))
  (bind _output_get (set `local.meshcomp` _asstatic_mesh_component))
  (for (_array_element _array_index) (`MeshComponent.GetMaterials` _output_get)
    (bind _asmaterial_instance_dynamic (cast `MaterialInstanceDynamic` _array_element)
      (:`then`
        (set `local.material` _asmaterial_instance_dynamic))
      (:`CastFailed`
        (bind _returnvalue (`PrimitiveComponent.CreateDynamicMaterialInstance` _output_get _array_index _array_element))
        (set `local.material` _returnvalue)))
    (`MaterialInstanceDynamic.SetScalarParameterValue` (`local.material`) "Alpha" Value)))

(fn `UserConstructionScript`)