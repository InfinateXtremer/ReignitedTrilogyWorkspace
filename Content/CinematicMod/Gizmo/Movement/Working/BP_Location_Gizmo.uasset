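; Translation gizmo actor that drags a target component along its X, Y or Z arrow with the mouse, destroying itself when the target actor is invalid.
; Each tick highlights arrows near the cursor through a material parameter and, when idle, follows the target's transform.
; Dragging intersects the mouse ray with a camera-oriented plane through the axis, then projects onto that axis minus the grab offset.
; Target physics simulation is suspended while dragging and restored on release.
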(event `self.ReceiveBeginPlay`
  (`parent.ReceiveBeginPlay`))

(event `self.ReceiveTick`
  (params (DeltaSeconds :type "Float (single-precision)"))
  (bind _targetcomponent (`self.TargetComponent`))
  (bind _currenttouchedcomponent (`self.CurrentTouchedComponent`))
  (`/Engine/EditorBlueprintResources/StandardMacros.IsValid` (`self.TargetActor`)
    (:`Is Valid`
      (`self.CalculateCameraDistanceFromGizmo`)
      (set `self.CurrentLocation` (`self.K2_GetActorLocation`))
      (`self.PickArrow` (`self.X`))
      (`self.PickArrow` (`self.Y`))
      (`self.PickArrow` (`self.Z`))
      (`/Engine/EditorBlueprintResources/StandardMacros.IsValid` _currenttouchedcomponent
        (:`Is Valid`
          (bind _newparam1 (`self.Movement` _currenttouchedcomponent))
          (`self.K2_SetActorLocation` _newparam1 false true)
          (`SceneComponent.K2_SetWorldLocation` (`self.TargetComponent`) _newparam1 false false)
          (bind _asmesh_component (cast `MeshComponent` (`self.TargetComponent`)))
          (`PrimitiveComponent.SetSimulatePhysics` _asmesh_component false))
        (:`Is Not Valid`
          (`self.K2_SetActorLocationAndRotation` (`SceneComponent.K2_GetComponentLocation` _targetcomponent) (`SceneComponent.K2_GetComponentRotation` _targetcomponent)))))
    (:`Is Not Valid`
      (`self.K2_DestroyActor`))))

(event `Key|LeftMouseButton` :consume false :overrideparent false
  (params (Key :type "Key Structure"))
  (:`Pressed`
    (set `self.Clicking` true)
    (set `self.CurrentLocation` (`self.K2_GetActorLocation`))
    (set `self.CurrentOffset` (`self.GetCurrentOffsetUnderMouse`))
    (`GameplayStatics.PlaySound2D` null)
    (`/Engine/EditorBlueprintResources/StandardMacros.DoOnce` false :!label _label
      (:`Completed`
        (set `self.WasSimulatingPhysics` (`SceneComponent.IsSimulatingPhysics` (`self.TargetComponent`) "None")))))
  (:`Released`
    (set `self.Clicking` false)
    (set `self.CurrentTouchedComponent` null)
    (bind _asmesh_component (cast `MeshComponent` (`self.TargetComponent`)))
    (`PrimitiveComponent.SetSimulatePhysics` _asmesh_component (`self.WasSimulatingPhysics`))
    (`GameplayStatics.PlaySound2D` null)
    (goto _label :!via `Reset`)))

(fn `Debug`
  (params (Center :type "Vector Structure") (LineColor :type "LinearColor Structure") (Distance :type "Float (double-precision)")))

(fn `Movement`
  (params (Component :type "PrimitiveComponent Object Reference"))
  (returns (NewParam1 :type "Vector Structure"))
  (locals (NewLocalVar_0 :type "PrimitiveComponent Object Reference") (curComponent :type "StaticMeshComponent Object Reference") (ForwardVector :type "Vector Structure" :default (0.0 0.0 0.0)))
  (bind _forwardvector (`local.ForwardVector`))
  (bind _asstatic_mesh_component (cast `StaticMeshComponent` Component))
  (bind _output_get (set `local.curComponent` _asstatic_mesh_component))
  (set `local.ForwardVector` (`SceneComponent.GetForwardVector` _output_get))
  (return (- (+ (`KismetMathLibrary.ProjectVectorOnToVector` (`self.Math` (`KismetMathLibrary.Cross_VectorVector` (`KismetMathLibrary.Cross_VectorVector` (`KismetMathLibrary.Normal` (- (`self.GetCameraPosition`) (`self.CurrentLocation`))) _forwardvector) _forwardvector)) (`local.ForwardVector`)) (`self.CurrentLocation`)) (`self.CurrentOffset`))))

(fn `PickArrow`
  (params (StaticMeshComp :type "StaticMeshComponent Object Reference"))
  (bind _returnvalue_x (`KismetMathLibrary.BreakVector` (`self.GetActorScale3D`)))
  (bind _returnvalue (`SceneComponent.GetForwardVector` StaticMeshComp))
  (bind _returnvalue_2 (`SceneComponent.K2_GetComponentLocation` StaticMeshComp))
  (bind _returnvalue_3 (* _returnvalue (* _returnvalue_x 100.0)))
  (bind _returnvalue_4 (<= (`KismetMathLibrary.GetPointDistanceToSegment` (`self.Math` (`KismetMathLibrary.Cross_VectorVector` (`KismetMathLibrary.Cross_VectorVector` (`KismetMathLibrary.Normal` (- (`self.GetCameraPosition`) (`self.CurrentLocation`))) _returnvalue) _returnvalue)) (0.0 0.0 0.0) _returnvalue_3) 5.0))
  (`KismetSystemLibrary.DrawDebugArrow` _returnvalue_2 (+ _returnvalue_3 _returnvalue_2) 0.0 (`KismetMathLibrary.Conv_VectorToLinearColor` _returnvalue))
  (if _returnvalue_4
    (`self.SetMaterialValue` StaticMeshComp 1.0)
    (if (and _returnvalue_4 (`self.Clicking`) (not (`KismetSystemLibrary.IsValid` (`self.CurrentTouchedComponent`))))
      (set `self.CurrentTouchedComponent` StaticMeshComp)
      (set `self.CurrentOffset` (`self.GetCurrentOffsetUnderMouse`)))
    (else
      ;[1 1 1] Unhighlight Selection
      (if (not (and (`self.Clicking`) (`KismetSystemLibrary.IsValid` (`self.CurrentTouchedComponent`))))
        (`self.SetMaterialValue` StaticMeshComp)))))

(fn `SetCurrentLocationAndOffset`)

(fn `SetMaterialValue`
  (params (Object :type "Object Object Reference") (Value :type "Float (double-precision)"))
  (locals (meshcomp :type "StaticMeshComponent Object Reference") (material :type "MaterialInstanceDynamic Object Reference"))
  (bind _asstatic_mesh_component (cast `StaticMeshComponent` Object))
  (bind _output_get (set `local.meshcomp` _asstatic_mesh_component))
  (bind _returnvalue (`PrimitiveComponent.GetMaterial` _output_get 0))
  (bind _asmaterial_instance_dynamic (cast `MaterialInstanceDynamic` _returnvalue)
    (:`then`
      (set `local.material` _asmaterial_instance_dynamic))
    (:`CastFailed`
      (bind _returnvalue_2 (`PrimitiveComponent.CreateDynamicMaterialInstance` _output_get 0 _returnvalue))
      (set `local.material` _returnvalue_2)))
  (`MaterialInstanceDynamic.SetScalarParameterValue` (`local.material`) "Alpha" Value))

(fn `UserConstructionScript`)