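; Base actor for the transform gizmos of a cinematic mod, each bound to a target component.
; On BeginPlay it stores the target's owner and tags itself with owner and component names for tracking.
; A differing transform mode spawns the location, rotation or scale gizmo on the same target and destroys this one; None only destroys.
; A helper function scales the gizmo by camera distance, while the interface getters are empty stubs.
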(event `self.ReceiveBeginPlay`
  (bind _targetcomponent (`self.TargetComponent`))
  (bind _returnvalue (`ActorComponent.GetOwner` _targetcomponent))
  ;[1 1 1] We add current target actors' name as tag to our gizmo to track them.
  (set `self.TargetActor` _returnvalue)
  (`KismetArrayLibrary.Array_Add` (`self.Tags`) (`KismetStringLibrary.Conv_StringToName` (`KismetStringLibrary.Concat_StrStr` (`KismetSystemLibrary.GetDisplayName` _returnvalue) (`KismetSystemLibrary.GetDisplayName` _targetcomponent)))))

(event `/Game/CinematicMod/Blueprints/Interfaces/BPI_HUD.IUpdateGizmoTransformMode`
  (params (Transformmode :type "/Game/CinematicMod/Gizmo/Movement/EGizmoTransformMode Enum" :default "NewEnumerator0"))
  (bind _targetcomponent (`self.TargetComponent`))
  (if (!= Transformmode (`self.GizmoType`))
    (switch `/Game/CinematicMod/Gizmo/Movement/EGizmoTransformMode` Transformmode
      (:`NewEnumerator0`
        (`|SpawnActorFromClass` "/Game/CinematicMod/Gizmo/Movement/Working/BP_Location_Gizmo.BP_Location_Gizmo_C" (`KismetMathLibrary.MakeTransform` (0.0 0.0 0.0)) "Undefined" "OverrideRootScale" null "NewEnumerator0" _targetcomponent null)
        (`self.K2_DestroyActor` :!label _label))
      (:`NewEnumerator1`
        (`|SpawnActorFromClass` "/Game/CinematicMod/Gizmo/Movement/Working/BP_Rotation_Gizmo.BP_Rotation_Gizmo_C" (`KismetMathLibrary.MakeTransform` (0.0 0.0 0.0)) "Undefined" "OverrideRootScale" null false "NewEnumerator1" _targetcomponent null)
        (goto _label))
      (:`NewEnumerator2`
        (`|SpawnActorFromClass` "/Game/CinematicMod/Gizmo/Movement/Working/BP_Scale.BP_Scale_C" (`KismetMathLibrary.MakeTransform` (0.0 0.0 0.0)) "Undefined" "OverrideRootScale" null "NewEnumerator0" _targetcomponent null)
        (goto _label))
      (:`NewEnumerator3`
        (`self.K2_DestroyActor`)))))

(fn `CalculateCameraDistanceFromGizmo`
  (`self.SetActorScale3D` (`KismetMathLibrary.Conv_DoubleToVector` (/ (`KismetMathLibrary.VSize` (- (`self.K2_GetActorLocation`) (`SceneComponent.K2_GetComponentLocation` (`PlayerCameraManager.TransformComponent` (`GameplayStatics.GetPlayerCameraManager` 0))))) 350.0))))

(fn `IGetActorData`
  (params (NewParam :type "Actor Object Reference"))
  (returns (ActorData :type String))
  (return ""))

(fn `IGetCinematicCamera`
  (returns (BP_CameraActor :type "/Game/CinematicMod/Blueprints/BP_CameraActor Object Reference"))
  (return null))

(fn `IGetCinematicWidget`
  (returns (CurrentWidget :type "/Game/CinematicMod/Blueprints/Widget/AdvancedUI Object Reference"))
  (return null))

(fn `IGetComponentData`
  (params (Component :type "ActorComponent Object Reference"))
  (returns (Data :type String))
  (return ""))

(fn `IGetRequestedBoolVariableValue`
  (params (variableName :type String))
  (returns (NewParam :type Boolean))
  (return false))

(fn `UserConstructionScript`)