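; Showcase actor for the cinematic mod's particle browser that displays a looping particle system through its own framing camera.
; UpdateParticle swaps the template and resets the tracked radius, while SetView makes the actor the player's view target, saving the previous one.
; Each tick eases the camera to a FOV-based distance from the largest bounds seen, nudges its initial rotation toward the effect and draws a debug bounding box.
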(event `self.ReceiveTick`
  (params (DeltaSeconds :type "Float (single-precision)"))
  (set `self.DeltaTime` DeltaSeconds)
  (`self.DebugVisualize`)
  (`self.CameraDistance`)
  (`self.UpdateRotation`)
  (add `ParticleSystemComponent.OnSystemFinished` (`self.ParticleSystem`) (delegate `CustomEvent_0`)))

(event `CustomEvent_0`
  (params (PSystem :type "ParticleSystemComponent Object Reference"))
  ;[1 1 1] Loop particle system
  (`ActorComponent.Activate` (`self.ParticleSystem`) true :!label _label))

(event `self.ReceiveBeginPlay`
  (set `self.InitialRotation` (`SceneComponent.K2_GetComponentRotation` (`self.Camera`))))

(event `self.ParticleSystem.OnSystemFinished`
  (params (PSystem :type "ParticleSystemComponent Object Reference"))
  ;[1 1 1] Loop particle system
  (goto _label))

(event `CameraDistance`
  (bind (_origin _boxextent _sphereradius) (`KismetSystemLibrary.GetComponentBounds` (`self.ParticleSystem`)))
  (if (> _sphereradius (`self.MaxSphereRadius`))
    (set `self.BoundingOriginOffset` (`KismetMathLibrary.InverseTransformLocation` (`self.GetTransform`) _origin)))
  (set `self.MaxSphereRadius` (`KismetMathLibrary.FMax` (`.SphereRadius` (`KismetSystemLibrary.GetComponentBounds` (`self.ParticleSystem`))) (`self.MaxSphereRadius`)))
  (set `self.CurrentLocation` (`SceneComponent.K2_GetComponentLocation` (`self.Camera`)))
  (set `self.TargetLocation` (+ (`KismetMathLibrary.TransformLocation` (`self.GetTransform`) (`self.BoundingOriginOffset`)) (* (`KismetMathLibrary.NegateVector` (`KismetMathLibrary.GetForwardVector` (`self.InitialRotation`))) (* (/ 1.0 (`KismetMathLibrary.DegCos` (/ (- 180.0 (`CameraComponent.FieldOfView` (`self.Camera`))) 2.0))) (`self.MaxSphereRadius`)))))
  (`SceneComponent.K2_SetWorldLocation` (`self.Camera`) (`KismetMathLibrary.VInterpTo` (`self.CurrentLocation`) (`self.TargetLocation`) (`self.DeltaTime`) 4.0) false false))

(event `UpdateRotation`
  ;[1 1 1] Rotation
  (set `self.TargetRotation` (`KismetMathLibrary.FindLookAtRotation` (`SceneComponent.K2_GetComponentLocation` (`self.Camera`)) (`KismetSystemLibrary.GetComponentBounds` (`self.ParticleSystem`))))
  (`SceneComponent.K2_SetWorldRotation` (`self.Camera`) (`KismetMathLibrary.RInterpTo` (`self.InitialRotation`) (`self.TargetRotation`) (`self.DeltaTime`) 2.0) false false))

(fn `DebugVisualize`
  (bind (_origin _boxextent) (`KismetSystemLibrary.GetComponentBounds` (`self.ParticleSystem`)))
  (`KismetSystemLibrary.DrawDebugBox` _origin _boxextent (struct :`R` 1.0 :`A` 1.0)))

(fn `SetView`
  (bind _returnvalue (`Controller.GetViewTarget` (`GameplayStatics.GetPlayerController` 0)))
  (if (!= _returnvalue self)
    (set `self.OriginalViewTarget` _returnvalue))
  (`PlayerController.SetViewTargetWithBlend` (`GameplayStatics.GetPlayerController` 0) self 0.0 "VTBlend_Linear" 0.0 false))

(fn `UpdateParticle`
  (params (NewTemplate :type "ParticleSystem Object Reference"))
  (set `self.MaxSphereRadius` 0.0)
  (`ParticleSystemComponent.SetTemplate` (`self.ParticleSystem`) NewTemplate))

(fn `UserConstructionScript`)