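; VisualCircleActor is a temporary sphere visual that shows a radius centered on the player character.
; UpdateCircleSize scales the Sphere uniformly from the given radius and moves the actor to player 0's current location.
; BeginPlay and each update restart a retriggerable delay, so the actor destroys itself once updates stop for DestructionTime.
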(event `self.ReceiveBeginPlay`
  (`self.TriggerDestruction`))

(event `UpdateCircleSize`
  (params (radius :type "Float (double-precision)"))
  (`SceneComponent.SetRelativeScale3D` (`self.Sphere`) (`KismetMathLibrary.Conv_DoubleToVector` (* radius 0.02)))
  (`self.K2_SetActorLocation` (`self.K2_GetActorLocation` (`GameplayStatics.GetPlayerCharacter` 0)))
  (`self.TriggerDestruction`))

(event `TriggerDestruction`
  (`KismetSystemLibrary.RetriggerableDelay` (`self.DestructionTime`))
  (`self.K2_DestroyActor`))

(fn `UserConstructionScript`)