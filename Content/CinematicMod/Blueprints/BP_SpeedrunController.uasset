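; Speedrun assist controller for CinematicMod that registers a menu keybind and shows the SpeedrunTools widget.
; CheckKeybinds adds SpeedrunMenu axis mappings for gamepad and keyboard at runtime when no CameraAxisLeftRight action mapping is found.
; ShowSpeedrunMenu creates the widget on first use, disabling look input and showing the cursor; later calls only toggle its visibility.
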(event `CheckKeybinds`
  (bind _returnvalue (`InputSettings.GetInputSettings`))
  ;[1 1 1] Speedrun Assist
  (if (== (`KismetArrayLibrary.Array_Length` (`InputSettings.GetActionMappingByName` (`InputSettings.GetInputSettings`) "CameraAxisLeftRight")) 0)
    (`InputSettings.AddAxisMapping` _returnvalue (make `InputAxisKeyMapping` "SpeedrunMenu" "Gamepad_DPad_Up") true)
    (`InputSettings.AddAxisMapping` _returnvalue (make `InputAxisKeyMapping` "SpeedrunMenu" "Multiply") true)))

(event `ShowSpeedrunMenu`
  (bind _playercontroller (`self.PlayerController`))
  (bind _speedrunui (`self.SpeedRunUI`)
    (:`then`
      (`Widget.SetVisibility` (`self.SpeedRunUI`) (select `bool` (not (`Widget.IsVisible` _speedrunui)) :`false` "Hidden" :`true` "Visible" :!type "ESlateVisibility Enum")))
    (:`else`
      (bind _returnvalue (`|CreateWidget` "/Game/CinematicMod/Blueprints/Widget/SpeedrunTools.SpeedrunTools_C" (`GameplayStatics.GetPlayerController` 0)))
      (bind _output_get (set `self.SpeedRunUI` _returnvalue))
      (`UserWidget.AddToViewport` _output_get 1)
      (`Controller.SetIgnoreLookInput` _playercontroller true)
      (set `PlayerController.bShowMouseCursor` true _playercontroller))))

(fn `UserConstructionScript`)