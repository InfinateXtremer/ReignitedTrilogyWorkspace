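; CinematicMod Blueprint library with two helper functions for converting array data.
; NameArrayToStringList converts each array element to a string and joins the results with a given separator.
; ParsePhasmidInventoryıtem turns an array of inventory item entries into a map from item type to quantity.
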(fn `NameArrayToStringList`
  (params (Array :type "Array of Name") (Separator :type String))
  (returns (OrderedString :type String))
  (locals (stringarray :type "Array of String"))
  (for _array_element Array
    (`KismetArrayLibrary.Array_Add` (`local.stringarray`) (`KismetStringLibrary.Conv_NameToString` _array_element)))
  (return (`KismetStringLibrary.JoinStringArray` (`local.stringarray`) Separator)))

(fn `ParsePhasmidInventoryıtem`
  (params (Array :type "Array of PhasmidInventoryItem Structure"))
  (returns (InventoryItemMap1 :type "Map of EInventoryType Enum to Integer"))
  (locals (InventoryItemMap :type "Map of EInventoryType Enum to Object Object Reference"))
  (for _array_element Array
    (bind (_itemtype _quantity) (break `PhasmidInventoryItem` _array_element))
    (`BlueprintMapLibrary.Map_Add` (`local.InventoryItemMap`) _itemtype _quantity))
  (return (`local.InventoryItemMap`)))