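; Posable character actor that mirrors a Character's skeletal mesh and current pose on a PoseableMesh, and can save and load poses as text.
; On BeginPlay it copies mesh and pose from the Character and tags itself with that character's name.
; CreatePoseData serializes each socket name's parent-relative transform into a joined string.
; ProcessData splits such data, skips '#' entries, and ParseBoneData recomposes each transform with its parent's in component space.
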(event `self.ReceiveBeginPlay`
  (bind _character (`self.Character`))
  (`/Engine/EditorBlueprintResources/StandardMacros.IsValid` _character
    (:`Is Valid`
      (`self.UpdateMesh` (`SkinnedMeshComponent.SkeletalMesh` (`Character.Mesh` _character)))
      (`KismetArrayLibrary.Array_AddUnique` (`self.Tags`) (`KismetStringLibrary.Conv_StringToName` (`KismetSystemLibrary.GetDisplayName` (`self.Character`))))
      (`PoseableMeshComponent.CopyPoseFromSkeletalComponent` (`self.PoseableMesh`) (`Character.Mesh` (`self.Character`))))))

(fn `CreatePoseData`
  (returns (PoseData :type String))
  (locals (PoseDataArray :type "Array of String") (Bonename :type Name) (ParentTransform :type "Transform Structure") (BoneTransform :type "Transform Structure"))
  (for _array_element (`SceneComponent.GetAllSocketNames` (`self.PoseableMesh`))
    (bind _output_get (set `local.Bonename` _array_element))
    (bind _returnvalue (`SkinnedMeshComponent.GetParentBone` (`self.PoseableMesh`) _output_get))
    (if (!= _returnvalue "None")
      (bind _returnvalue_2 (`PoseableMeshComponent.GetBoneTransformByName` (`self.PoseableMesh`) _returnvalue "ComponentSpace"))
      (set `local.ParentTransform` _returnvalue_2))
    (bind _returnvalue_3 (`PoseableMeshComponent.GetBoneTransformByName` (`self.PoseableMesh`) (`local.Bonename`) "ComponentSpace"))
    (set `local.BoneTransform` _returnvalue_3)
    (`KismetArrayLibrary.Array_Add` (`local.PoseDataArray`) (`KismetTextLibrary.Conv_TextToString` (`self.CreateTextData` (`local.Bonename`) (`KismetMathLibrary.ComposeTransforms` (`local.BoneTransform`) (`KismetMathLibrary.InvertTransform` (`local.ParentTransform`)))))))
  (return (`KismetStringLibrary.JoinStringArray` (`local.PoseDataArray`) " \n")))

(fn `ParseBoneData`
  (params (BoneData :type String))
  (locals (BoneName :type String) (BoneLocalLocation :type "Vector Structure" :default (0.0 0.0 0.0)) (BoneLocalRotation :type "Rotator Structure" :default (struct)) (BoneLocalScale :type "Vector Structure" :default (0.0 0.0 0.0)) (parentlocation :type "Vector Structure" :default (0.0 0.0 0.0)) (ParentTransform :type "Transform Structure") (boneTransform :type "Transform Structure"))
  (bind (_lefts _rights) (`KismetStringLibrary.Split` BoneData "|"))
  (bind _poseablemesh (`self.PoseableMesh`))
  (bind (_lefts_2 _rights_2) (`KismetStringLibrary.Split` _rights "|"))
  (bind (_lefts_3 _rights_3) (`KismetStringLibrary.Split` _rights_2 "|"))
  (if (not (`KismetStringLibrary.StartsWith` BoneData "#"))
    (bind _output_get (set `local.BoneName` _lefts))
    (bind _returnvalue (`SkinnedMeshComponent.GetParentBone` _poseablemesh (`KismetStringLibrary.Conv_StringToName` _output_get)))
    (if (!= _returnvalue "None")
      (bind _returnvalue_2 (`PoseableMeshComponent.GetBoneTransformByName` _poseablemesh _returnvalue "ComponentSpace"))
      (set `local.ParentTransform` _returnvalue_2))
    (set `local.boneTransform` (`KismetMathLibrary.MakeTransform` (`KismetStringLibrary.Conv_StringToVector` _lefts_2) (`KismetStringLibrary.Conv_StringToRotator` _lefts_3) (`KismetStringLibrary.Conv_StringToVector` _rights_3)))
    (`PoseableMeshComponent.SetBoneTransformByName` (`self.PoseableMesh`) (`KismetStringLibrary.Conv_StringToName` (`local.BoneName`)) (`KismetMathLibrary.ComposeTransforms` (`local.boneTransform`) (`local.ParentTransform`)) "ComponentSpace")))

(fn `ProcessData`
  (params (Data :type String))
  (for _array_element (`KismetStringLibrary.ParseIntoArray` Data " \n")
    (`self.ParseBoneData` _array_element)))

(fn `UpdateMesh`
  (params (NewMesh :type "SkeletalMesh Object Reference"))
  (`SkinnedMeshComponent.SetSkinnedAssetAndUpdate` (`self.PoseableMesh`) NewMesh false))

(fn `UserConstructionScript`)