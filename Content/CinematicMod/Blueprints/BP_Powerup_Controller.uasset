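; Spyro mod controller that grants powerups (breaths, fairy kiss, superflame, magma invincibility, supercharge, free flight) via hotkeys.
; BeginPlay adds any missing number-key and numpad action mappings at runtime.
; Presses apply GameplayEffects to the player, sustained by looping timers, usually setting body materials unless WithoutSkin; supercharge and packaged-only free flight stack without clearing others.
; C clears powerups; other keys heal, damage or set materials.
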(event `self.ReceiveBeginPlay`
  (`self.CheckIceBreath`)
  (`self.CheckFairyKiss`)
  (`self.CheckSuperFlame`)
  (`self.CheckSpikedIceBreath`)
  (`self.CheckMagma`)
  (`self.CheckSupercharge`)
  (`self.CheckFreeFlight`))

(event `CheckIceBreath`
  (bind _returnvalue (`InputSettings.GetInputSettings`))
  ;[1 1 1] Spyro3 Ice Breath
  (if (== (`KismetArrayLibrary.Array_Length` (`InputSettings.GetActionMappingByName` (`InputSettings.GetInputSettings`) "Ice Breath")) 0)
    (`InputSettings.AddActionMapping` _returnvalue (make `InputActionKeyMapping` "Ice Breath" "One") true)
    (`InputSettings.AddActionMapping` _returnvalue (make `InputActionKeyMapping` "Ice Breath" "NumPadOne") true)))

(event `CheckFairyKiss`
  (bind _returnvalue (`InputSettings.GetInputSettings`))
  ;[1 1 1] Fairy Kiss
  (if (== (`KismetArrayLibrary.Array_Length` (`InputSettings.GetActionMappingByName` (`InputSettings.GetInputSettings`) "Fairy Kiss")) 0)
    (`InputSettings.AddActionMapping` _returnvalue (make `InputActionKeyMapping` "Fairy Kiss" "Two") true)
    (`InputSettings.AddActionMapping` _returnvalue (make `InputActionKeyMapping` "Fairy Kiss" "NumPadTwo") true)))

(event `CheckSuperFlame`
  (bind _returnvalue (`InputSettings.GetInputSettings`))
  ;[1 1 1] SuperFlame
  (if (== (`KismetArrayLibrary.Array_Length` (`InputSettings.GetActionMappingByName` (`InputSettings.GetInputSettings`) "SuperFlame")) 0)
    (`InputSettings.AddActionMapping` _returnvalue (make `InputActionKeyMapping` "SuperFlame" "Three") true)
    (`InputSettings.AddActionMapping` _returnvalue (make `InputActionKeyMapping` "SuperFlame" "NumPadThree") true)))

(event `CheckSpikedIceBreath`
  (bind _returnvalue (`InputSettings.GetInputSettings`))
  ;[1 1 1] Spyro 2 Ice Breath
  (if (== (`KismetArrayLibrary.Array_Length` (`InputSettings.GetActionMappingByName` (`InputSettings.GetInputSettings`) "SpikedIceBreath")) 0)
    (`InputSettings.AddActionMapping` _returnvalue (make `InputActionKeyMapping` "SpikedIceBreath" "Four") true)
    (`InputSettings.AddActionMapping` _returnvalue (make `InputActionKeyMapping` "SpikedIceBreath" "NumPadFour") true)))

(event `CheckMagma`
  (bind _returnvalue (`InputSettings.GetInputSettings`))
  ;[1 1 1] Magma
  (if (== (`KismetArrayLibrary.Array_Length` (`InputSettings.GetActionMappingByName` (`InputSettings.GetInputSettings`) "Magma")) 0)
    (`InputSettings.AddActionMapping` _returnvalue (make `InputActionKeyMapping` "Magma" "Five") true)
    (`InputSettings.AddActionMapping` _returnvalue (make `InputActionKeyMapping` "Magma" "NumPadFive") true)))

(event `CheckSupercharge`
  (bind _returnvalue (`InputSettings.GetInputSettings`))
  ;[1 1 1] Supercharge
  (if (== (`KismetArrayLibrary.Array_Length` (`InputSettings.GetActionMappingByName` (`InputSettings.GetInputSettings`) "Supercharge")) 0)
    (`InputSettings.AddActionMapping` _returnvalue (make `InputActionKeyMapping` "Supercharge" "Six") true)
    (`InputSettings.AddActionMapping` _returnvalue (make `InputActionKeyMapping` "Supercharge" "NumPadSix") true)))

(event `CheckFreeFlight`
  (bind _returnvalue (`InputSettings.GetInputSettings`))
  ;[1 1 1] Freeflight
  (if (== (`KismetArrayLibrary.Array_Length` (`InputSettings.GetActionMappingByName` (`InputSettings.GetInputSettings`) "FreeFlight")) 0)
    (`InputSettings.AddActionMapping` _returnvalue (make `InputActionKeyMapping` "FreeFlight" "NumPadSeven") true)
    (`InputSettings.AddActionMapping` _returnvalue (make `InputActionKeyMapping` "FreeFlight" "Seven") true)))

(event `Key|C` :consume false :overrideparent false
  (params (Key :type "Key Structure"))
  ;[1 1 1] Clear Fires and Use Normal Breath
  (:`Pressed`
    (`self.ClearEffects`)
    (bind _asbp_cps1999_playable (cast `/CPS1999_Spyro/Blueprints/BP_CPS1999_Playable` (`GameplayStatics.GetPlayerPawn` 0)))
    (`PrimitiveComponent.SetMaterial` (`Character.Mesh` _asbp_cps1999_playable) 0 null)
    (bind _returnvalue (`AbilitySystemBlueprintLibrary.GetAbilitySystemComponent` _asbp_cps1999_playable))
    (`AbilitySystemComponent.RemoveActiveGameplayEffectBySourceEffect` _returnvalue "/CharacterCommon/AbilitySystem/GameplayEffects/Spyro/GE_SpyroSuperFlyEnabled.GE_SpyroSuperFlyEnabled_C" null -1)
    (`AbilitySystemComponent.RemoveActiveGameplayEffectBySourceEffect` _returnvalue "/CharacterCommon/AbilitySystem/GameplayEffects/Spyro/GE_SpyroSuperChargeForceOn.GE_SpyroSuperChargeForceOn_C" null -1)
    (`KismetSystemLibrary.K2_ClearAndInvalidateTimerHandle` (`self.FreeFlightTimer`))))

(event `IceBreath`
  ;[1 1 1] Ice Breath
  (if (not (`self.WithoutSkin?`)) :!label _label
    (`PrimitiveComponent.SetMaterial` (`Character.Mesh` (stale `InputAction|Ice Breath` _asbp_cps1999_playable)) 0 null))
  (bind _returnvalue (`AbilitySystemComponent.BP_ApplyGameplayEffectToSelf` :`self` (`AbilitySystemBlueprintLibrary.GetAbilitySystemComponent` (stale `InputAction|Ice Breath` _asbp_cps1999_playable)) :`GameplayEffectClass` "/CharacterCommon/AbilitySystem/GameplayEffects/Spyro/GE_SpyroIceFireEnabled.GE_SpyroIceFireEnabled_C" :`Level` 10.0)))

(event `InputAction|Ice Breath` :consume false :overrideparent false
  (params (Key :type "Key Structure"))
  ;[1 1 1] Ice Breath
  (:`Pressed`
    (bind _asbp_cps1999_playable (cast `/CPS1999_Spyro/Blueprints/BP_CPS1999_Playable` (`GameplayStatics.GetPlayerPawn` 0)))
    (`self.ClearEffects`)
    (bind _returnvalue (`KismetSystemLibrary.K2_SetTimer` null "IceBreath" 2.0 true))
    (set `self.IceBreathTimer` _returnvalue)
    (goto _label)))

(event `ClearEffects`
  (`|ExecutionSequence`
    (:`then_0`
      (`AbilitySystemComponent.RemoveActiveGameplayEffect` (`AbilitySystemBlueprintLibrary.GetAbilitySystemComponent` (stale `InputAction|Ice Breath` _asbp_cps1999_playable)) (stale `IceBreath` _returnvalue) -1))
    (:`then_1`
      (`AbilitySystemComponent.RemoveActiveGameplayEffect` (`AbilitySystemBlueprintLibrary.GetAbilitySystemComponent` (stale `InputAction|Fairy Kiss` _asbp_cps1999_playable)) (stale `Ragefire` _returnvalue) -1))
    (:`then_2`
      (bind _returnvalue (`AbilitySystemBlueprintLibrary.GetAbilitySystemComponent` (stale `InputAction|SuperFlame` _asbp_cps1999_playable)))
      (`AbilitySystemComponent.RemoveActiveGameplayEffect` _returnvalue (stale `Superflame` _returnvalue) -1)
      (`AbilitySystemComponent.RemoveActiveGameplayEffectBySourceEffect` _returnvalue "/CharacterCommon/Abilities/GameplayEffects/GE_Enable_PermanentSuperFire.GE_Enable_PermanentSuperFire_C" null -1))
    (:`then_3`
      (`AbilitySystemComponent.RemoveActiveGameplayEffect` (`AbilitySystemBlueprintLibrary.GetAbilitySystemComponent` (stale `InputAction|SpikedIceBreath` _asbp_cps1999_playable)) (stale `Spikes` _returnvalue) -1))
    (:`then_4`
      (`AbilitySystemComponent.RemoveActiveGameplayEffect` (`AbilitySystemBlueprintLibrary.GetAbilitySystemComponent` (stale `InputAction|Magma` _asbp_cps1999_playable)) (stale `Magma` _returnvalue) -1))
    (:`then_5`
      (`AbilitySystemComponent.RemoveActiveGameplayEffect` (`AbilitySystemBlueprintLibrary.GetAbilitySystemComponent` (stale `InputAction|Supercharge` _asbp_cps1999_playable)) (stale `SuperCharge` _returnvalue) -1))
    (:`then_6`
      (`KismetSystemLibrary.K2_ClearAndInvalidateTimerHandle` (`self.SuperChargeTimer`) :!label _label_2)
      (`KismetSystemLibrary.K2_ClearAndInvalidateTimerHandle` (`self.MagmaTimer`))
      (`KismetSystemLibrary.K2_ClearAndInvalidateTimerHandle` (`self.SpikesTimer`))
      (`KismetSystemLibrary.K2_ClearAndInvalidateTimerHandle` (`self.SuperflameTimer`))
      (`KismetSystemLibrary.K2_ClearAndInvalidateTimerHandle` (`self.RagefireTimer`))
      (`KismetSystemLibrary.K2_ClearAndInvalidateTimerHandle` (`self.IceBreathTimer`)))))

(event `Ragefire`
  ;[1 1 1] Fairy Kiss
  (if (not (`self.WithoutSkin?`)) :!label _label_3
    (`PrimitiveComponent.SetMaterial` (`Character.Mesh` (stale `InputAction|Fairy Kiss` _asbp_cps1999_playable)) 0 null))
  (bind _returnvalue (`AbilitySystemComponent.BP_ApplyGameplayEffectToSelf` :`self` (`AbilitySystemBlueprintLibrary.GetAbilitySystemComponent` (stale `InputAction|Fairy Kiss` _asbp_cps1999_playable)) :`GameplayEffectClass` "/CharacterCommon/AbilitySystem/GameplayEffects/Spyro/GE_SpyroRageFireEnabled.GE_SpyroRageFireEnabled_C" :`Level` 10.0)))

(event `InputAction|Fairy Kiss` :consume false :overrideparent false
  (params (Key :type "Key Structure"))
  ;[1 1 1] Fairy Kiss
  (:`Pressed`
    (bind _asbp_cps1999_playable (cast `/CPS1999_Spyro/Blueprints/BP_CPS1999_Playable` (`GameplayStatics.GetPlayerPawn` 0)))
    (`self.ClearEffects`)
    (bind _returnvalue (`KismetSystemLibrary.K2_SetTimer` null "Ragefire" 2.0 true))
    (set `self.RagefireTimer` _returnvalue)
    (goto _label_3)))

(event `Clear Timers`
  (goto _label_2))

(event `Superflame`
  ;[1 1 1] Superflame
  (if (not (`self.WithoutSkin?`)) :!label _label_4
    (`PrimitiveComponent.SetMaterial` (`Character.Mesh` (stale `InputAction|SuperFlame` _asbp_cps1999_playable)) 0 "/CPS1999_Spyro/Materials/MI_CPS1999_Spyro_Fireball.MI_CPS1999_Spyro_Fireball"))
  (bind _returnvalue (`AbilitySystemComponent.BP_ApplyGameplayEffectToSelf` :`self` (`AbilitySystemBlueprintLibrary.GetAbilitySystemComponent` (stale `InputAction|SuperFlame` _asbp_cps1999_playable)) :`GameplayEffectClass` "/CharacterCommon/AbilitySystem/GameplayEffects/Spyro/GE_SpyroSuperFireEnabled.GE_SpyroSuperFireEnabled_C" :`Level` 10.0)))

(event `InputAction|SuperFlame` :consume false :overrideparent false
  (params (Key :type "Key Structure"))
  ;[1 1 1] Superflame
  (:`Pressed`
    (bind _asbp_cps1999_playable (cast `/CPS1999_Spyro/Blueprints/BP_CPS1999_Playable` (`GameplayStatics.GetPlayerPawn` 0)))
    (`self.ClearEffects`)
    (bind _returnvalue (`KismetSystemLibrary.K2_SetTimer` null "Superflame" 2.0 true))
    (set `self.SuperflameTimer` _returnvalue)
    (goto _label_4)))

(event `ApplyFreeflight`
  (if (`KismetSystemLibrary.IsPackagedForDistribution`)
    ;[1 1 1] FreeFlight
    (`AbilitySystemComponent.BP_ApplyGameplayEffectToSelf` :`self` (`AbilitySystemBlueprintLibrary.GetAbilitySystemComponent` (stale `InputAction|FreeFlight` _asbp_cps1999_playable)) :`GameplayEffectClass` "/CharacterCommon/AbilitySystem/GameplayEffects/Spyro/GE_SpyroSuperFlyEnabled.GE_SpyroSuperFlyEnabled_C" :`Level` 10.0 :!label _label_5)
    (bind _returnvalue (`KismetSystemLibrary.K2_SetTimer` null "ApplyFreeflight" 2.0 true))
    (set `self.FreeFlightTimer` _returnvalue)))

(event `InputAction|FreeFlight` :consume false :overrideparent false
  (params (Key :type "Key Structure"))
  ;[1 1 1] FreeFlight
  (:`Pressed`
    (if (`KismetSystemLibrary.IsPackagedForDistribution`)
      (bind _asbp_cps1999_playable (cast `/CPS1999_Spyro/Blueprints/BP_CPS1999_Playable` (`GameplayStatics.GetPlayerPawn` 0)))
      (goto _label_5))))

(event `Spikes`
  ;[1 1 1] Ice Breath Spikes
  (if (not (`self.WithoutSkin?`)) :!label _label_6
    (`PrimitiveComponent.SetMaterial` (`Character.Mesh` (stale `InputAction|SpikedIceBreath` _asbp_cps1999_playable)) 0 null))
  (bind _returnvalue (`AbilitySystemComponent.BP_ApplyGameplayEffectToSelf` :`self` (`AbilitySystemBlueprintLibrary.GetAbilitySystemComponent` (stale `InputAction|SpikedIceBreath` _asbp_cps1999_playable)) :`GameplayEffectClass` "/CharacterCommon/AbilitySystem/GameplayEffects/Spyro/GE_SpyroIceBreathEnabled.GE_SpyroIceBreathEnabled_C" :`Level` 10.0)))

(event `InputAction|SpikedIceBreath` :consume false :overrideparent false
  (params (Key :type "Key Structure"))
  ;[1 1 1] Ice Breath Spikes
  (:`Pressed`
    (bind _asbp_cps1999_playable (cast `/CPS1999_Spyro/Blueprints/BP_CPS1999_Playable` (`GameplayStatics.GetPlayerPawn` 0)))
    (`self.ClearEffects`)
    (bind _returnvalue (`KismetSystemLibrary.K2_SetTimer` null "Spikes" 2.0 true))
    (set `self.SpikesTimer` _returnvalue)
    (goto _label_6)))

(event `Key|Add` :consume false :overrideparent false
  (params (Key :type "Key Structure"))
  ;[1 1 1] Heal
  (:`Pressed`
    (bind _asbp_cps1999_playable (cast `/CPS1999_Spyro/Blueprints/BP_CPS1999_Playable` (`GameplayStatics.GetPlayerPawn` 0)))
    (`AbilitySystemComponent.BP_ApplyGameplayEffectToSelf` :`self` (`AbilitySystemBlueprintLibrary.GetAbilitySystemComponent` _asbp_cps1999_playable) :`GameplayEffectClass` "/CharacterCommon/Abilities/GameplayEffects/GE_BasicHeal.GE_BasicHeal_C" :`Level` 1.0)))

(event `Key|Subtract` :consume false :overrideparent false
  (params (Key :type "Key Structure"))
  ;[1 1 1] Heal
  (:`Pressed`
    (bind _asbp_cps1999_playable (cast `/CPS1999_Spyro/Blueprints/BP_CPS1999_Playable` (`GameplayStatics.GetPlayerPawn` 0)))
    (`AbilitySystemComponent.BP_ApplyGameplayEffectToSelf` :`self` (`AbilitySystemBlueprintLibrary.GetAbilitySystemComponent` _asbp_cps1999_playable) :`GameplayEffectClass` "/CharacterCommon/Abilities/GameplayEffects/GE_BasicDamage.GE_BasicDamage_C" :`Level` 1.0)))

(event `Magma`
  ;[1 1 1] Magma
  (bind _returnvalue (`AbilitySystemComponent.BP_ApplyGameplayEffectToSelf` :`self` (`AbilitySystemBlueprintLibrary.GetAbilitySystemComponent` (stale `InputAction|Magma` _asbp_cps1999_playable)) :`GameplayEffectClass` "/CharacterCommon/Abilities/GameplayEffects/GE_Invincibility.GE_Invincibility_C" :`Level` 10.0)))

(event `InputAction|Magma` :consume false :overrideparent false
  (params (Key :type "Key Structure"))
  ;[1 1 1] Magma
  (:`Pressed`
    (bind _asbp_cps1999_playable (cast `/CPS1999_Spyro/Blueprints/BP_CPS1999_Playable` (`GameplayStatics.GetPlayerPawn` 0)))
    (`self.ClearEffects`)
    (bind _returnvalue (`KismetSystemLibrary.K2_SetTimer` null "Magma" 2.0 true))
    (set `self.MagmaTimer` _returnvalue)
    (if (not (`self.WithoutSkin?`))
      (`PrimitiveComponent.SetMaterial` (`Character.Mesh` _asbp_cps1999_playable) 0 null))))

(event `SuperCharge`
  ;[1 1 1] Supercharge
  (bind _returnvalue (`AbilitySystemComponent.BP_ApplyGameplayEffectToSelf` :`self` (`AbilitySystemBlueprintLibrary.GetAbilitySystemComponent` (stale `InputAction|Supercharge` _asbp_cps1999_playable)) :`GameplayEffectClass` "/CharacterCommon/AbilitySystem/GameplayEffects/Spyro/GE_SpyroSuperChargeForceOn.GE_SpyroSuperChargeForceOn_C" :`Level` 10.0 :!label _label_7)))

(event `InputAction|Supercharge` :consume false :overrideparent false
  (params (Key :type "Key Structure"))
  ;[1 1 1] Supercharge
  (:`Pressed`
    (bind _asbp_cps1999_playable (cast `/CPS1999_Spyro/Blueprints/BP_CPS1999_Playable` (`GameplayStatics.GetPlayerPawn` 0)))
    (bind _returnvalue (`KismetSystemLibrary.K2_SetTimer` null "SuperCharge" 2.0 true))
    (set `self.SuperChargeTimer` _returnvalue)
    (if (`self.WithoutSkin?`)
      (goto _label_7)
      (else
        (`PrimitiveComponent.SetMaterial` (`Character.Mesh` _asbp_cps1999_playable) 0 null)
        (goto _label_7)))))

(event `Key|Seven` :consume false :overrideparent false
  (params (Key :type "Key Structure"))
  ;[1 1 1] Nightmare Mode
)

(event `Key|NumPadSeven` :consume false :overrideparent false
  (params (Key :type "Key Structure"))
  ;[1 1 1] Nightmare Mode
)

(event `Key|NumPadEight` :consume false :overrideparent false
  (params (Key :type "Key Structure"))
  (:`Pressed`
    (bind _asbp_cps1999_playable (cast `/CPS1999_Spyro/Blueprints/BP_CPS1999_Playable` (`GameplayStatics.GetPlayerPawn` 0)))
    (`PrimitiveComponent.SetMaterial` (`Character.Mesh` _asbp_cps1999_playable) 0 null)))

(event `Key|NumPadNine` :consume false :overrideparent false
  (params (Key :type "Key Structure"))
  (:`Pressed`
    (bind _asbp_cps1999_playable (cast `/CPS1999_Spyro/Blueprints/BP_CPS1999_Playable` (`GameplayStatics.GetPlayerPawn` 0)))
    (`PrimitiveComponent.SetMaterial` (`Character.Mesh` _asbp_cps1999_playable) 0 null)))

(fn `UserConstructionScript`)