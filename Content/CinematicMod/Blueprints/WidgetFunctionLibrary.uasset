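; Blueprint function library of helpers for the CinematicMod widgets: tag checks, text search, selection highlighting and save-slot access.
; ToggleSelection tints the button and toggles custom depth on the actor's mesh component.
; GetSaveGame loads or creates a BP_CinematicSave, while SaveGame always writes the loaded object and returns the newly created one, even though only one exists per branch.
; UpdateUIColors is an empty stub.
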(fn `CheckForSelectedTag`
  (params (Actor :type "Actor Object Reference") (TagToFind :type String))
  (returns (`Selected?` :type Boolean))
  (bind _tags (`Actor.Tags` Actor))
  (return (`KismetArrayLibrary.Array_IsValidIndex` _tags (`KismetArrayLibrary.Array_Find` _tags (`KismetStringLibrary.Conv_StringToName` TagToFind)))))

(fn `GetSaveGame`
  (params (SlotName :type String :default "cache"))
  (returns (`BP Cinematic Save` :type "/Game/CinematicMod/Blueprints/BP_CinematicSave Object Reference"))
  (bind _returnvalue (`GameplayStatics.DoesSaveGameExist` SlotName))
  (if _returnvalue
    (bind _returnvalue_2 (`GameplayStatics.LoadGameFromSlot` SlotName))
    (bind _asbp_cinematic_save (cast `/Game/CinematicMod/Blueprints/BP_CinematicSave` _returnvalue_2))
    (return _asbp_cinematic_save)
    (else
      (bind _returnvalue_3 (`GameplayStatics.CreateSaveGameObject` "/Game/CinematicMod/Blueprints/BP_CinematicSave.BP_CinematicSave_C"))
      (`GameplayStatics.SaveGameToSlot` _returnvalue_3 SlotName)
      (return _returnvalue_3))))

(fn `SaveGame`
  (params (SlotName :type String :default "cache"))
  (returns (`BP Cinematic Save` :type "/Game/CinematicMod/Blueprints/BP_CinematicSave Object Reference"))
  (bind _returnvalue (`GameplayStatics.DoesSaveGameExist` SlotName))
  (if _returnvalue
    (bind _returnvalue_2 (`GameplayStatics.LoadGameFromSlot` SlotName))
    (else
      (bind _returnvalue_3 (`GameplayStatics.CreateSaveGameObject` "/Game/CinematicMod/Blueprints/BP_CinematicSave.BP_CinematicSave_C"))))
  (`GameplayStatics.SaveGameToSlot` _returnvalue_2 SlotName)
  (return _returnvalue_3))

(fn `Search`
  (params (`Search Parameter` :type "Text (by ref)") (Empty :type Boolean) (Text :type "Text (by ref)"))
  (returns (Found :type Boolean))
  (if Empty
    (return true)
    (else
      (return (`KismetStringLibrary.Contains` (`KismetTextLibrary.Conv_TextToString` Text) (`KismetTextLibrary.Conv_TextToString` `Search Parameter`))))))

(fn `ToggleSelection`
  (params (`Selected?` :type Boolean) (Button :type "Button Object Reference") (Actor :type "Actor Object Reference"))
  (bind _returnvalue (`Actor.GetComponentByClass` Actor "/Script/Engine.MeshComponent"))
  (`Button.SetBackgroundColor` Button (select `bool` `Selected?` :`false` (struct :`R` 1.0 :`G` 1.0 :`B` 1.0 :`A` 1.0) :`true` (struct :`R` 0.064803 :`G` 0.332452 :`A` 1.0) :!type "LinearColor Structure"))
  (`/Engine/EditorBlueprintResources/StandardMacros.IsValid` _returnvalue
    (:`Is Valid`
      (`PrimitiveComponent.SetRenderCustomDepth` _returnvalue `Selected?`))))

(fn `UpdateUIColors`)