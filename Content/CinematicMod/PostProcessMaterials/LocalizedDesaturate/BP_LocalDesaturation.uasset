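; BP_LocalDesaturation is a placeable actor that applies a localized post-process effect, by its name desaturation, to a box-shaped region of the level.
; Its construction script creates a dynamic instance of LocalPP_Blend_Inst and feeds it the Box component's world location and scaled extents.
; The instance is added to the PostProcess component as a full-weight blendable, leaving the spatial masking to the material; no runtime logic runs.
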(fn `UserConstructionScript`
  (bind _box (`self.Box`))
  (bind (_returnvalue_x _returnvalue_y _returnvalue_z) (`KismetMathLibrary.BreakVector` (`BoxComponent.GetScaledBoxExtent` _box)))
  (bind _returnvalue (`KismetMaterialLibrary.CreateDynamicMaterialInstance` "/Game/CinematicMod/PostProcessMaterials/LocalizedDesaturate/LocalPP_Blend_Inst.LocalPP_Blend_Inst"))
  (`MaterialInstanceDynamic.SetVectorParameterValue` _returnvalue "BoxCenter" (`KismetMathLibrary.Conv_VectorToLinearColor` (`SceneComponent.K2_GetComponentLocation` _box)))
  (`MaterialInstanceDynamic.SetScalarParameterValue` _returnvalue "BoxX" _returnvalue_x)
  (`MaterialInstanceDynamic.SetScalarParameterValue` _returnvalue "BoxY" _returnvalue_y)
  (`MaterialInstanceDynamic.SetScalarParameterValue` _returnvalue "BoxZ" _returnvalue_z)
  (`PostProcessComponent.AddOrUpdateBlendable` (`self.PostProcess`) _returnvalue 1.0))