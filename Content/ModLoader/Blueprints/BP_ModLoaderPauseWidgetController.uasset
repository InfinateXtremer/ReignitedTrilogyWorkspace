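; BP_ModLoaderPauseWidgetController injects a "MOD LOADER" button into the game's pause menu at runtime.
; Every Tick it finds all UI_Pause widgets and scans their VerticalBox0 children for that button's text, avoiding duplicates.
; When missing, it adds a UI_Pause_Button, then after a short delay plays its BeginFocus animation and overlays a filling UI_Modloader_Button on its text overlay.
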(event `self.ReceiveTick`
  (params (DeltaSeconds :type "Float (single-precision)"))
  (bind _foundwidgets (`WidgetBlueprintLibrary.GetAllWidgetsOfClass` "/UserInterface/MenuScreens/UI_Pause.UI_Pause_C" false))
  (for _array_element _foundwidgets
    (set `self.founddesiredChild?` false)
    (bind _verticalbox_0 (`/UserInterface/MenuScreens/UI_Pause.VerticalBox_0` _array_element))
    (for _index (range (+ (`PanelWidget.GetChildrenCount` _verticalbox_0) 1))
      (bind _asui_pause_button (cast `/UserInterface/MenuScreens/UI_Pause_Button` (`PanelWidget.GetChildAt` _verticalbox_0 _index)))
      (if (`KismetTextLibrary.EqualEqual_TextText` (`/UserInterface/MenuScreens/UI_Pause_Button.Text` _asui_pause_button) "MOD LOADER")
        (set `self.founddesiredChild?` true)))
    (if (not (`self.founddesiredChild?`))
      (bind _returnvalue (`|CreateWidget` "/UserInterface/MenuScreens/UI_Pause_Button.UI_Pause_Button_C" null "MOD LOADER"))
      (`PanelWidget.AddChild` _verticalbox_0 _returnvalue)
      (`KismetSystemLibrary.Delay` 0.2)
      (`UserWidget.PlayAnimation` _returnvalue (`/UserInterface/MenuScreens/UI_Pause_Button.BeginFocus` _returnvalue) 0.0 1 "Forward" 1.0)
      (bind _returnvalue_2 (`|GenericCreateObject` "/Game/ModLoader/Blueprints/Widgets/UI_Modloader_Button.UI_Modloader_Button_C" self))
      (bind _returnvalue_3 (`Overlay.AddChildToOverlay` (`/UserInterface/MenuScreens/UI_Pause_Button.OverlayText` _returnvalue) _returnvalue_2))
      (`OverlaySlot.SetHorizontalAlignment` _returnvalue_3 "HAlign_Fill")
      (`OverlaySlot.SetVerticalAlignment` _returnvalue_3 "VAlign_Fill"))))

(fn `UserConstructionScript`)