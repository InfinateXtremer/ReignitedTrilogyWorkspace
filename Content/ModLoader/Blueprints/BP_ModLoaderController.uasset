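; Mod loader controller that creates and toggles the ModViewer menu widget through hotkeys.
; F10, F5 and Multiply always trigger the toggle, while K does so only in builds not packaged for distribution.
; Showing runs garbage collection, creates a fresh widget and enables the mouse cursor; hiding removes it and hides the cursor.
; BeginPlay pre-creates the menu, removing it after a short delay, and debug prints report UI state.
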(event `Key|K` :consume false :overrideparent false
  (params (Key :type "Key Structure"))
  ;[1 1 1] ModLoaderVisibility
  (:`Pressed`
    (if (not (`KismetSystemLibrary.IsPackagedForDistribution`))
      (`self.ShowModLoaderWidget` :!label _label))))

(event `self.ReceiveBeginPlay`
  ;[1 1 1] ModLoaderVisibility
  (`self.CreateModLoaderMenu` false))

(event `Key|F10` :consume false :overrideparent false
  (params (Key :type "Key Structure"))
  ;[1 1 1] ModLoaderVisibility
  (:`Pressed`
    (goto _label)))

(event `Key|F5` :consume false :overrideparent false
  (params (Key :type "Key Structure"))
  ;[1 1 1] ModLoaderVisibility
  (:`Pressed`
    (goto _label)))

(event `Key|Multiply` :consume false :overrideparent false
  (params (Key :type "Key Structure"))
  ;[1 1 1] ModLoaderVisibility
  (:`Pressed`
    (goto _label)))

(event `ShowModLoaderWidget`
  (bind _modmenu (`self.ModMenu`))
  ;[1 1 1] ModLoaderVisibility
  (`/Engine/EditorBlueprintResources/StandardMacros.IsValid` (`self.ModMenu`)
    (:`Is Valid`
      (if (`Widget.IsVisible` (`self.ModMenu`))
        (`Widget.SetVisibility` _modmenu "Collapsed")
        (set `PlayerController.bShowMouseCursor` false (`GameplayStatics.GetPlayerController` 0))
        (`Widget.RemoveFromParent` _modmenu)
        (`/Game/ModLoader/Blueprints/Widgets/Utility/BF_PrintText.BF_PrintString` "UI Removed")
        (else
          (`KismetSystemLibrary.CollectGarbage` :!label _label_2)
          (bind _returnvalue (`|CreateWidget` "/Game/ModLoader/Blueprints/ModViewer.ModViewer_C"))
          (`/Engine/EditorBlueprintResources/StandardMacros.IsValid` _returnvalue
            (:`Is Valid`
              (`/Game/ModLoader/Blueprints/Widgets/Utility/BF_PrintText.BF_PrintString` "UI Created")
              (bind _output_get (set `self.ModMenu` _returnvalue))
              (`UserWidget.AddToViewport` _output_get 0)
              (set `PlayerController.bShowMouseCursor` true (`GameplayStatics.GetPlayerController` 0))
              (`/Game/ModLoader/Blueprints/Widgets/Utility/BF_PrintText.BF_PrintString` "UI Added to HUD"))
            (:`Is Not Valid`
              (`/Game/ModLoader/Blueprints/Widgets/Utility/BF_PrintText.BF_PrintString` "UI Creation Failed"))))))
    (:`Is Not Valid`
      (goto _label_2))))

(event `CreateModLoaderMenu`
  (params (`Show?` :type Boolean))
  (bind _modmenu (`self.ModMenu`))
  ;[1 1 1] ModLoaderVisibility
  (`|ExecutionSequence`
    (:`then_0`
      (goto _label_2))
    (:`then_1`
      (if `Show?`
        (`UserWidget.AddToViewport` _modmenu 0)
        (else
          (`UserWidget.AddToViewport` _modmenu 0)
          (`KismetSystemLibrary.Delay` 0.2)
          (`Widget.RemoveFromParent` _modmenu))))))

(fn `UserConstructionScript`)